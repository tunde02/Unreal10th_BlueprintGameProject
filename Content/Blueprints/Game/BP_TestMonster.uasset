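; BP_TestMonster is a test monster that moves along an array of waypoint actors supplied through SetWaypoints, once StartMove is called.
; Tick moves it at constant speed toward the current waypoint, advancing the index when within a small squared 2D distance.
; Passing the last waypoint costs one HP and loops back to the second waypoint.
; At zero HP it notifies the wave manager given by SetWaveManager and destroys itself.
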(event `/Game/Blueprints/Game/BPI_WaypointMovable.StartMove`
  (set `self.bMoving` true))

(event `/Game/Blueprints/Game/BPI_WaypointMovable.SetWaypoints`
  (params (InWaypoints :type "Array of Actor Object Reference (by ref)"))
  (set `self.Waypoints` InWaypoints))

(event `self.ReceiveTick`
  (params (DeltaSeconds :type "Float (single-precision)"))
  (if (`self.bMoving`)
    (`self.MoveToCurrentWaypoint` DeltaSeconds)))

(event `MoveToCurrentWaypoint`
  (params (InDeltaSeconds :type "Float (double-precision)"))
  (`self.K2_SetActorLocation` (`KismetMathLibrary.VInterpTo_Constant` (`self.K2_GetActorLocation`) (`self.K2_GetActorLocation` (`|GetArrayItem` (`self.Waypoints`) (`self.CurrentWaypointIndex`))) InDeltaSeconds (`self.MoveSpeed`)))
  (`self.CheckWaypointIndex`))

(event `CheckWaypointIndex`
  (bind _returnvalue (`KismetArrayLibrary.Array_Length` (`self.Waypoints`)))
  (if (< (`KismetMathLibrary.Vector_Distance2DSquared` (`self.K2_GetActorLocation`) (`self.K2_GetActorLocation` (`|GetArrayItem` (`self.Waypoints`) (`self.CurrentWaypointIndex`)))) 5.0)
    (bind _result (`/Engine/EditorBlueprintResources/StandardMacros.IncrementInt` (`self.CurrentWaypointIndex`))
      (:`  `
        (if (>= _result _returnvalue)
          (bind _result_2 (`/Engine/EditorBlueprintResources/StandardMacros.DecrementInt` (`self.Hp`))
            (:`  `
              (if (<= _result_2 0)
                (`/Game/Blueprints/Game/BPI_WaveManager.OnMonsterDeath` (`self.BPI_WaveManager`))
                (`self.K2_DestroyActor`)
                (else
                  (set `self.CurrentWaypointIndex` (+ (mod (`self.CurrentWaypointIndex`) _returnvalue) 1)))))))))))

(event `/Game/Blueprints/Game/BPI_Monster.SetWaveManager`
  (params (InWaveManager :type "/Game/Blueprints/Game/BPI_WaveManager Interface"))
  (set `self.BPI_WaveManager` InWaveManager))

(fn `UserConstructionScript`)