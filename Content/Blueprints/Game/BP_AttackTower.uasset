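; Attack tower Blueprint that attacks its current targets through BPCAttackComponent, using runtime stats and combined base and enchanted attack effects.
; Looping timers tick two maps of timed effects and enchants, expiring entries, with pause/resume logic for idle timers.
; Stat updates run effect modifiers through BPCEffectComponent, resize the range collider and selection circle, then broadcast the change.
; Periodic effects are dispatched by interval, but their type switch is empty.
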(event `/Game/Blueprints/Interface/BPI_Tower.SetTowerData`
  (params (InTowerData :type "/Game/Blueprints/Data/Tower/ST_TowerData Structure"))
  (`self.HandleSetTowerData` InTowerData))

(event `/Game/Blueprints/Interface/BPI_EffectReceiver.AddEffect`
  (params (InEffectType :type "/Game/Blueprints/Data/Effect/E_EffectType Enum" :default "NewEnumerator0") (InEffectData :type "/Game/Blueprints/Data/Effect/ST_EffectData Structure"))
  (`/Game/Blueprints/Game/BPC_EffectComponent.AddEffect` (`self.BPC_EffectComponent`) InEffectType InEffectData)
  (`/Game/Blueprints/Game/BPC_EffectComponent.TryResumeActiveEffectTickTimer` (`self.BPC_EffectComponent`) (`self.ActiveEffectMap`) (`self.ActiveEffectMapTickTimer`)))

(event `/Game/Blueprints/Interface/BPI_EffectReceiver.SetActiveEffectMap`
  (params (InActiveEffectMap :type "Map of /Game/Blueprints/Data/Effect/E_EffectType Enum to /Game/Blueprints/Data/Effect/ST_EffectData Structure" :default _))
  (set `self.ActiveEffectMap` InActiveEffectMap))

(event `/Game/Blueprints/Interface/BPI_Tower.Place`
  (params (InIsBench :type Boolean) (InGrid :type "Actor Object Reference"))
  (`parent.Place` InIsBench InGrid))

(event `/Game/Blueprints/Interface/BPI_EffectReceiver.UpdateRuntimeStat`
  (`self.HandleUpdateRuntimeStat`))

(event `/Game/Blueprints/Interface/BPI_EnchantEffectReceiver.AddEnchantEffect`
  (params (InEffectType :type "/Game/Blueprints/Data/Effect/E_EffectType Enum" :default "NewEnumerator0") (InEnchantEffectData :type "/Game/Blueprints/Data/Effect/ST_EnchantEffectData Structure"))
  (bind _activeenchanteffectmapticktimer (`self.ActiveEnchantEffectMapTickTimer`))
  (`BlueprintMapLibrary.Map_Add` (`self.ActiveEnchantEffectMap`) InEffectType InEnchantEffectData)
  (`self.ApplyEnchantEffect` InEnchantEffectData)
  (if (and (`KismetSystemLibrary.K2_IsTimerPausedHandle` _activeenchanteffectmapticktimer) (> (`BlueprintMapLibrary.Map_Length` (`self.ActiveEnchantEffectMap`)) 0))
    (`KismetSystemLibrary.K2_UnPauseTimerHandle` _activeenchanteffectmapticktimer)))

(fn `Action`
  (locals (TotalAttackEffects :type "Array of /Game/Blueprints/Data/Effect/ST_EffectData Structure"))
  (bind (_commondata _statdata _attackdata) (break `/Game/Blueprints/Data/Tower/ST_TowerData` (`self.TowerData`)))
  (bind (_attackpower _attackrate _range _targetcount _piercecount) (break `/Game/Blueprints/Data/Tower/ST_RuntimeTowerStatData` (`self.RuntimeStat`)))
  (if (`KismetArrayLibrary.Array_IsNotEmpty` (`self.CurrentTargets`))
    ; 공격 이펙트 구현 부분
    (`self.DrawDebugLineToTarget`)
    (bind _values (`BlueprintMapLibrary.Map_Values` (`self.EnchantedAttackEffectMap`)))
    (bind _output_get (set `local.TotalAttackEffects` _values))
    (`KismetArrayLibrary.Array_Append` _output_get (`.AttackEffects_21_69AB2C1F4C9193AEE821E5B6A30A4ECB` (break `/Game/Blueprints/Data/Tower/ST_AttackData` _attackdata)))
    (`/Game/Blueprints/Game/BPC_AttackComponent.Attack` (`self.BPC_AttackComponent`) _attackdata (`self.CurrentTargets`) (`.Current_10_8823095F44368B8BD7DA00B9AF4F8038` (break `/Game/Blueprints/Data/Effect/ST_FloatStat` _attackpower)) (`.Current_11_2E47CF62452CAF1771442281E93C8672` (break `/Game/Blueprints/Data/Effect/ST_IntStat` _piercecount)) (`SceneComponent.K2_GetComponentLocation` (`self.ProjectileSpawnPoint`)) (`local.TotalAttackEffects`))
    (`self.UpdateNextAvailableTime`)))

(fn `ApplyEnchantEffect`
  (params (InEnchantEffect :type "/Game/Blueprints/Data/Effect/ST_EnchantEffectData Structure"))
  (bind (_enchanteffect _attackeffect) (break `/Game/Blueprints/Data/Effect/ST_EnchantEffectData` InEnchantEffect))
  (`BlueprintMapLibrary.Map_Add` (`self.EnchantedAttackEffectMap`) (`.EffectType_29_192DAD4A459898673A1966BCF28039AD` (break `/Game/Blueprints/Data/Effect/ST_EffectData` _attackeffect)) _attackeffect))

(fn `ApplyPeriodicEffect`
  (params (InEffectData :type "/Game/Blueprints/Data/Effect/ST_EffectData Structure"))
  (switch `/Game/Blueprints/Data/Effect/E_EffectType` (`.EffectType_29_192DAD4A459898673A1966BCF28039AD` (break `/Game/Blueprints/Data/Effect/ST_EffectData` InEffectData))))

(fn `GetActiveEffectMap`
  (returns (OutActiveEffecetMap :type "Map of /Game/Blueprints/Data/Effect/E_EffectType Enum to /Game/Blueprints/Data/Effect/ST_EffectData Structure"))
  (return (`self.ActiveEffectMap`)))

(fn `HandleSetTowerData`
  (params (InTowerData :type "/Game/Blueprints/Data/Tower/ST_TowerData Structure"))
  (bind (_attacktype _projectile _projectilespeed _damageradius _attackeffects) (break `/Game/Blueprints/Data/Tower/ST_AttackData` (`.AttackData_13_87AA181541E6A0B586485CB0061B034F` (break `/Game/Blueprints/Data/Tower/ST_TowerData` InTowerData))))
  (`parent.HandleSetTowerData` InTowerData)
  (set `self.AttackType` _attacktype)
  (for _array_element _attackeffects
    (`BlueprintMapLibrary.Map_Add` (`self.OwnAttackEffectMap`) (`.EffectType_29_192DAD4A459898673A1966BCF28039AD` (break `/Game/Blueprints/Data/Effect/ST_EffectData` _array_element)) _array_element))
  (bind _returnvalue (`KismetSystemLibrary.K2_SetTimerDelegate` (`|CreateDelegate` :!event `TickActiveEffectMap`) (`self.EffectTick`) true))
  (bind _output_get (set `self.ActiveEffectMapTickTimer` _returnvalue))
  (bind _returnvalue_2 (`KismetSystemLibrary.K2_SetTimerDelegate` (`|CreateDelegate` :!event `TickActiveEnchantEffectMap`) (`self.EffectTick`) true))
  (bind _output_get_2 (set `self.ActiveEnchantEffectMapTickTimer` _returnvalue_2))
  (`KismetSystemLibrary.K2_PauseTimerHandle` _output_get_2))

(fn `HandleUpdateRuntimeStat`
  (bind _runtimestat (`self.RuntimeStat`))
  (bind _runtimestat_2 (`self.RuntimeStat`))
  (bind _runtimestat_3 (`self.RuntimeStat`))
  (bind _runtimestat_4 (`self.RuntimeStat`))
  (bind _runtimestat_5 (`self.RuntimeStat`))
  (bind _bpc_effectcomponent (`self.BPC_EffectComponent`))
  (bind (_attackpower _attackrate _range _targetcount _piercecount) (break `/Game/Blueprints/Data/Tower/ST_RuntimeTowerStatData` (`self.RuntimeStat`)))
  (bind (_attackpower_2 _attackrate_2 _range_2 _targetcount_2 _piercecount_2) (break `/Game/Blueprints/Data/Tower/ST_RuntimeTowerStatData` (`self.RuntimeStat`)))
  (bind (_base _current) (break `/Game/Blueprints/Data/Effect/ST_IntStat` _piercecount_2))
  (bind (_base_2 _current_2) (break `/Game/Blueprints/Data/Effect/ST_IntStat` _targetcount_2))
  (bind (_base_3 _current_3) (break `/Game/Blueprints/Data/Effect/ST_FloatStat` _attackpower_2))
  (bind (_base_4 _current_4) (break `/Game/Blueprints/Data/Effect/ST_FloatStat` _range_2))
  (bind (_base_5 _current_5) (break `/Game/Blueprints/Data/Effect/ST_FloatStat` _attackrate_2))
  (set `self.RuntimeStat` (make `/Game/Blueprints/Data/Tower/ST_RuntimeTowerStatData` (make `/Game/Blueprints/Data/Effect/ST_FloatStat` _base_3 _current_3) (make `/Game/Blueprints/Data/Effect/ST_FloatStat` _base_5 _current_5) (make `/Game/Blueprints/Data/Effect/ST_FloatStat` _base_4 _current_4) (make `/Game/Blueprints/Data/Effect/ST_IntStat` _base_2 _current_2) (make `/Game/Blueprints/Data/Effect/ST_IntStat` _base _current)))
  (bind (_keypin _valuepin) (`|MapForEach` (`self.ActiveEffectMap`))
    (:`then`
      (if true
        (switch `/Game/Blueprints/Data/Effect/E_StatType` (`.TargetStat_26_2399818F449D049BD491519515109832` (break `/Game/Blueprints/Data/Effect/ST_EffectData` _valuepin))
          (:`NewEnumerator0`
            (bind _outfloatstat (`/Game/Blueprints/Game/BPC_EffectComponent.AddModifierToFloatStat` _bpc_effectcomponent _attackpower _valuepin))
            (setmembers `/Game/Blueprints/Data/Tower/ST_RuntimeTowerStatData` :`StructRef` (`self.RuntimeStat`) :`AttackPower` _outfloatstat))
          (:`NewEnumerator1`
            (bind _outfloatstat_2 (`/Game/Blueprints/Game/BPC_EffectComponent.AddModifierToFloatStat` _bpc_effectcomponent _attackrate _valuepin))
            (setmembers `/Game/Blueprints/Data/Tower/ST_RuntimeTowerStatData` :`StructRef` (`self.RuntimeStat`) :`AttackRate` _outfloatstat_2))
          (:`NewEnumerator2`
            (bind _outfloatstat_3 (`/Game/Blueprints/Game/BPC_EffectComponent.AddModifierToFloatStat` _bpc_effectcomponent _range _valuepin))
            (setmembers `/Game/Blueprints/Data/Tower/ST_RuntimeTowerStatData` :`StructRef` (`self.RuntimeStat`) :`Range` _outfloatstat_3))
          (:`NewEnumerator3`
            (bind _outintstat (`/Game/Blueprints/Game/BPC_EffectComponent.AddModifierToIntStat` _bpc_effectcomponent _targetcount _valuepin))
            (setmembers `/Game/Blueprints/Data/Tower/ST_RuntimeTowerStatData` :`StructRef` (`self.RuntimeStat`) :`TargetCount` _outintstat))
          (:`NewEnumerator4`
            (bind _outintstat_2 (`/Game/Blueprints/Game/BPC_EffectComponent.AddModifierToIntStat` _bpc_effectcomponent _piercecount _valuepin))
            (setmembers `/Game/Blueprints/Data/Tower/ST_RuntimeTowerStatData` :`StructRef` (`self.RuntimeStat`) :`PierceCount` _outintstat_2)))))
    (:`CompletedPin`
      (`|ExecutionSequence`
        (:`then_0`
          (bind _outfloatstat_4 (`/Game/Blueprints/Game/BPC_EffectComponent.CalculateFloatStatCurrent` (`self.BPC_EffectComponent`) (`.AttackPower_28_2FB15F5042532A850C5FCF81A6040443` (break `/Game/Blueprints/Data/Tower/ST_RuntimeTowerStatData` _runtimestat_2))))
          (bind _structout (setmembers `/Game/Blueprints/Data/Tower/ST_RuntimeTowerStatData` :`StructRef` _runtimestat_2 :`AttackPower` _outfloatstat_4))
          (set `self.RuntimeStat` _structout))
        (:`then_1`
          (bind _outfloatstat_5 (`/Game/Blueprints/Game/BPC_EffectComponent.CalculateFloatStatCurrent` (`self.BPC_EffectComponent`) (`.AttackRate_29_2759D1F74AF0AA7105D4A6875A6697DD` (break `/Game/Blueprints/Data/Tower/ST_RuntimeTowerStatData` _runtimestat_3))))
          (bind _structout_2 (setmembers `/Game/Blueprints/Data/Tower/ST_RuntimeTowerStatData` :`StructRef` _runtimestat_3 :`AttackRate` _outfloatstat_5))
          (set `self.RuntimeStat` _structout_2))
        (:`then_2`
          (bind _outfloatstat_6 (`/Game/Blueprints/Game/BPC_EffectComponent.CalculateFloatStatCurrent` (`self.BPC_EffectComponent`) (`.Range_30_9C4464FF40E92343355B06A8A01E3A59` (break `/Game/Blueprints/Data/Tower/ST_RuntimeTowerStatData` _runtimestat_4))))
          (bind _structout_3 (setmembers `/Game/Blueprints/Data/Tower/ST_RuntimeTowerStatData` :`StructRef` _runtimestat_4 :`Range` _outfloatstat_6))
          (set `self.RuntimeStat` _structout_3)
          (bind _outrange (`self.GetRange`))
          (`SphereComponent.SetSphereRadius` (`self.RangeCollider`) _outrange true)
          (bind _returnvalue (/ (* _outrange 2.0) 100.0))
          (`SceneComponent.SetRelativeScale3D` (`self.SelectionCircle`) (`KismetMathLibrary.MakeVector` _returnvalue _returnvalue 1.0)))
        (:`then_3`
          (bind _outintstat_3 (`/Game/Blueprints/Game/BPC_EffectComponent.CalculateIntStatCurrent` (`self.BPC_EffectComponent`) (`.TargetCount_31_06E8D423489240A3AE6872B5E4B09F7D` (break `/Game/Blueprints/Data/Tower/ST_RuntimeTowerStatData` _runtimestat_5))))
          (bind _structout_4 (setmembers `/Game/Blueprints/Data/Tower/ST_RuntimeTowerStatData` :`StructRef` _runtimestat_5 :`TargetCount` _outintstat_3))
          (set `self.RuntimeStat` _structout_4))
        (:`then_4`
          (bind _outintstat_4 (`/Game/Blueprints/Game/BPC_EffectComponent.CalculateIntStatCurrent` (`self.BPC_EffectComponent`) (`.PierceCount_32_DBAB17EE49E41A240ADC718A3D2B3004` (break `/Game/Blueprints/Data/Tower/ST_RuntimeTowerStatData` _runtimestat))))
          (bind _structout_5 (setmembers `/Game/Blueprints/Data/Tower/ST_RuntimeTowerStatData` :`StructRef` _runtimestat :`PierceCount` _outintstat_4))
          (set `self.RuntimeStat` _structout_5))
        (:`then_5`
          (`self.OnRuntimeStatUpdated` self))))))

(fn `TickActiveEffectMap`
  (locals (CurrentEffectType :type "/Game/Blueprints/Data/Effect/E_EffectType Enum") (CurrentEffectData :type "/Game/Blueprints/Data/Effect/ST_EffectData Structure") (CurrentEffectCategory :type "/Game/Blueprints/Data/Effect/E_EffectCategory Enum") (CurrentDuration :type "Float (double-precision)") (CurrentInterval :type "Float (double-precision)") (CurrentElapsedTime :type "Float (double-precision)") (CurrentTotalElapsedTime :type "Float (double-precision)") (ExpiredEffects :type "Array of /Game/Blueprints/Data/Effect/E_EffectType Enum") (bShouldUpdateRuntimeStat :type Boolean))
  (bind (_keypin _valuepin) (`|MapForEach` (`self.ActiveEffectMap`))
    (:`then`
      (set `local.CurrentEffectType` _keypin)
      (bind _output_get (set `local.CurrentEffectData` _valuepin))
      (bind (_effecttype _effectcategory _effecttrigger _targetstat _modifiertype _value _duration _interval _elapsedtime _totalelapsedtime) (break `/Game/Blueprints/Data/Effect/ST_EffectData` _output_get))
      (set `local.CurrentEffectCategory` _effectcategory)
      (`|ExecutionSequence`
        (:`then_0`
          (set `local.CurrentDuration` _duration))
        (:`then_1`
          (set `local.CurrentInterval` _interval))
        (:`then_2`
          (if true
            (set `local.CurrentElapsedTime` (+ _elapsedtime (`self.EffectTick`)))))
        (:`then_3`
          (set `local.CurrentTotalElapsedTime` (+ _totalelapsedtime (`self.EffectTick`)))
          (if (> (`local.CurrentDuration`) (`local.CurrentTotalElapsedTime`))
            (if (`|EnumEquality` "NewEnumerator2" (`local.CurrentEffectCategory`))
              (if (>= (`local.CurrentElapsedTime`) (`local.CurrentInterval`))
                (bind _output_get_2 (set `local.CurrentElapsedTime` (- (`local.CurrentElapsedTime`) (`local.CurrentInterval`))))
                (bind _structout (setmembers `/Game/Blueprints/Data/Effect/ST_EffectData` :`StructRef` (`local.CurrentEffectData`) :`ElapsedTime` _output_get_2 :`TotalElapsedTime` (`local.CurrentTotalElapsedTime`)))
                (`BlueprintMapLibrary.Map_Add` (`self.ActiveEffectMap`) (`local.CurrentEffectType`) _structout)
                ; Tower.Tick() ->
                ; EffectComponent.ApplyPeriodicEffect() ->
                ; Tower.ApplyPeriodicEffect() 구조임
                (`self.ApplyPeriodicEffect` _structout)
                (else
                  (bind _structout_2 (setmembers `/Game/Blueprints/Data/Effect/ST_EffectData` :`StructRef` (`local.CurrentEffectData`) :`ElapsedTime` (`local.CurrentElapsedTime`) :`TotalElapsedTime` (`local.CurrentTotalElapsedTime`) :!label _label))
                  (`BlueprintMapLibrary.Map_Add` (`self.ActiveEffectMap`) (`local.CurrentEffectType`) _structout_2)))
              (else
                (goto _label)))
            (else
              (`KismetArrayLibrary.Array_Add` (`local.ExpiredEffects`) (`local.CurrentEffectType`)))))))
    (:`CompletedPin`
      (for _array_element (`local.ExpiredEffects`)
        (if (`|EnumEquality` (`.EffectCategory_12_8B9226C74EA0972C36E0D19B1BE55C05` (break `/Game/Blueprints/Data/Effect/ST_EffectData` (`BlueprintMapLibrary.Map_Find` (`self.ActiveEffectMap`) _array_element))) "NewEnumerator0")
          (set `local.bShouldUpdateRuntimeStat` true)
          (`BlueprintMapLibrary.Map_Remove` (`self.ActiveEffectMap`) _array_element)))
      (if (`local.bShouldUpdateRuntimeStat`)
        (`self.UpdateRuntimeStat`)
        (`/Game/Blueprints/Game/BPC_EffectComponent.TryPauseActiveEffectTickTimer` (`self.BPC_EffectComponent`) (`self.ActiveEffectMap`) (`self.ActiveEffectMapTickTimer`))))))

(fn `TickActiveEnchantEffectMap`
  (locals (CurrentEnchantedAttackEffectType :type "/Game/Blueprints/Data/Effect/E_EffectType Enum") (CurrentEnchantedAttackEffectData :type "/Game/Blueprints/Data/Effect/ST_EnchantEffectData Structure") (CurrentDuration :type "Float (double-precision)") (CurrentTotalElapsedTime :type "Float (double-precision)") (ExpiredEffects :type "Array of /Game/Blueprints/Data/Effect/E_EffectType Enum"))
  (bind (_effecttype _effectcategory _effecttrigger _targetstat _modifiertype _value _duration _interval _elapsedtime) (break `/Game/Blueprints/Data/Effect/ST_EffectData` (`.EnchantEffect_20_C1B0BAD0487CD8EA109814B0C806C8CC` (break `/Game/Blueprints/Data/Effect/ST_EnchantEffectData` (`local.CurrentEnchantedAttackEffectData`)))))
  (bind (_keypin _valuepin) (`|MapForEach` (`self.ActiveEnchantEffectMap`))
    (:`then`
      (set `local.CurrentEnchantedAttackEffectType` _keypin)
      (bind _output_get (set `local.CurrentEnchantedAttackEffectData` _valuepin))
      (bind (_effecttype_2 _effectcategory_2 _effecttrigger_2 _targetstat_2 _modifiertype_2 _value_2 _duration_2 _interval_2 _elapsedtime_2 _totalelapsedtime) (break `/Game/Blueprints/Data/Effect/ST_EffectData` (`.EnchantEffect_20_C1B0BAD0487CD8EA109814B0C806C8CC` (break `/Game/Blueprints/Data/Effect/ST_EnchantEffectData` _output_get))))
      (set `local.CurrentDuration` _duration_2)
      (set `local.CurrentTotalElapsedTime` (+ (`self.EffectTick`) _totalelapsedtime))
      (if (not (<= (`local.CurrentDuration`) (`local.CurrentTotalElapsedTime`)))
        (bind _structout (setmembers `/Game/Blueprints/Data/Effect/ST_EnchantEffectData` :`StructRef` (`local.CurrentEnchantedAttackEffectData`) :`EnchantEffect` (make `/Game/Blueprints/Data/Effect/ST_EffectData` _effecttype _effectcategory _effecttrigger _targetstat _modifiertype _value _duration _interval _elapsedtime (`local.CurrentTotalElapsedTime`))))
        (`BlueprintMapLibrary.Map_Add` (`self.ActiveEnchantEffectMap`) (`local.CurrentEnchantedAttackEffectType`) _structout)
        (else
          (`KismetArrayLibrary.Array_Add` (`local.ExpiredEffects`) (`local.CurrentEnchantedAttackEffectType`)))))
    (:`CompletedPin`
      (for _array_element (`local.ExpiredEffects`)
        (bind (_enchanteffect _attackeffect) (break `/Game/Blueprints/Data/Effect/ST_EnchantEffectData` (`BlueprintMapLibrary.Map_Find` (`self.ActiveEnchantEffectMap`) _array_element)))
        (`BlueprintMapLibrary.Map_Remove` (`self.EnchantedAttackEffectMap`) (`.EffectType_29_192DAD4A459898673A1966BCF28039AD` (break `/Game/Blueprints/Data/Effect/ST_EffectData` _attackeffect)))
        (`BlueprintMapLibrary.Map_Remove` (`self.ActiveEnchantEffectMap`) (`.EffectType_29_192DAD4A459898673A1966BCF28039AD` (break `/Game/Blueprints/Data/Effect/ST_EffectData` _enchanteffect))))
      (if (and (`KismetSystemLibrary.K2_IsTimerActiveHandle` (`self.ActiveEnchantEffectMapTickTimer`)) (`BlueprintMapLibrary.Map_IsEmpty` (`self.ActiveEnchantEffectMap`)))
        (`KismetSystemLibrary.K2_PauseTimerHandle` (struct))))))

(fn `UserConstructionScript`
  (`parent.UserConstructionScript`))