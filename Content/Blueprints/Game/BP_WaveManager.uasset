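; Wave manager that spawns monster waves from a data table and decides when the stage is cleared or failed.
; Looping timers alternate intermissions with waves, spawning through a monster factory component and sending monsters along waypoints.
; Live monster count triggers a warning near its limit and failure beyond it, as does a 60-second last-wave timeout on Tick.
; Clearing requires all waves finished and no monsters left; debug keys start, stop, pause and resume waves.
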(event Custom|StartWave
  (Development|PrintString (Utilities|String|BuildString(Integer) "" "Wave " (+ (Variables|Default|GetCurrentWaveIndex) 1) " 시작"))
  (CallFunction|SpawnMonster)
  (bind _returnvalue (Utilities|Time|SetTimerbyEvent (EventDispatchers|CreateEvent :!event Custom|SpawnMonster) (Variables|Default|GetCurrentWaveInterval) true))
  (Variables|Default|SetWaveTimer _returnvalue))

(event Custom|SpawnMonster
  (if (> (Variables|Default|GetCurrentWaveRemainingCount) 0)
    (bind _outspawnedmonster (Default|SpawnMonsterbyName (Variables|Default|GetBPC_MonsterFactory) (Variables|Default|GetCurrentWaveMonsterType) (Transformation|GetActorTransform (Variables|Default|GetSpawnLocation))))
    (Utilities|FlowControl|Sequence
      (:then_0
        (Class|BPIWaypointMovable|SetWaypoints(Message) _outspawnedmonster (Variables|Default|GetWaypoints)))
      (:then_1
        (Class|BPIWaypointMovable|StartMove(Message) _outspawnedmonster))
      (:then_2
        (CallFunction|OnMonsterSpawn)
        (bind _result (Math|Integer|DecrementInt (Variables|Default|GetCurrentWaveRemainingCount))
          (:%20%20
            (Development|PrintString (Utilities|String|BuildString(Integer) "" "남은 소환할 몬스터 수 : " _result))))))
    (else
      (CallFunction|StopWave)
      (CallFunction|StartIntermission))))

(event Custom|OnMonsterDeath
  (Math|Integer|DecrementInt (Variables|Default|GetMonsterCount)
    (:%20%20
      (CallFunction|CheckStageCleared))))

(event Custom|OnMonsterSpawn
  (Math|Integer|IncrementInt (Variables|Default|GetMonsterCount)
    (:%20%20
      (if (> (Variables|Default|GetMonsterCount) (* (Variables|Default|GetMonsterCountLimit) 0.8))
        (Default|CallOnMonsterCountWarning))
      (CallFunction|CheckStageFailed))))

(event Custom|Initialize
  (bind _outrownames (DataTable|GetDataTableRowNames (Variables|Default|GetWaveInfoDataTable)))
  (for _array_element _outrownames
    (bind _returnvalue (Utilities|GetDataTableRow (Variables|Default|GetWaveInfoDataTable) _array_element)
      (:then
        (Utilities|Array|Add (Variables|Default|GetWaveInfoList) _returnvalue))))
  (Variables|Default|SetTotalWaveCount (Utilities|Array|Length (Variables|Default|GetWaveInfoList)))
  (CallFunction|StartIntermission))

(event Custom|StopWave
  (Development|PrintString "WaveManager - StopWave()")
  (Utilities|Time|ClearandInvalidateTimerbyHandle (Variables|Default|GetWaveTimer)))

(event Custom|PauseWave
  (Development|PrintString "WaveManager - PauseWave()")
  (Utilities|Time|PauseTimerbyHandle (Variables|Default|GetWaveTimer)))

(event Custom|StartIntermission
  ;[0.15 0.15 0.15 0.5] 웨이브 시작점
  (Development|PrintString "쉬는 시간 10초 시작")
  (bind _returnvalue (Utilities|Time|SetTimerbyEvent (delegate Custom|SetNextWaveInfo) (Variables|Default|GetIntermissionTime)))
  (Variables|Default|SetIntermissionTimer _returnvalue)
  (bind _returnvalue_2 (Utilities|Time|SetTimerbyEvent (delegate Custom|PrintRemainingTime) 1.0 true)))

(event Custom|SetWaveInfo
  (bind _waveinfolist (Variables|Default|GetWaveInfoList))
  (bind _currentwaveindex (Variables|Default|GetCurrentWaveIndex))
  (bind _output (Utilities|Array|Get(acopy) _waveinfolist _currentwaveindex))
  (bind (_monstername _count _interval) (Utilities|Struct|BreakST_WaveInfo _output))
  (if (Utilities|Array|IsValidIndex _waveinfolist _currentwaveindex)
    (Utilities|FlowControl|Sequence
      (:then_0
        (Variables|Default|SetCurrentWaveMonsterType _monstername))
      (:then_1
        (Variables|Default|SetCurrentWaveRemainingCount _count))
      (:then_2
        (Variables|Default|SetCurrentWaveInterval _interval))
      (:then_3
        (CallFunction|StartWave)
        (Default|CallOnWaveIndexUpdate (Variables|Default|GetCurrentWaveIndex))))
    (elif (>= (Variables|Default|GetCurrentWaveIndex) (Variables|Default|GetTotalWaveCount))
      (Variables|Default|SetbWaveFinished true)
      (Development|PrintString "웨이브 끝남." true true "(R=0.000000,G=1.000000,B=0.000000,A=1.000000)")
      (CallFunction|CheckStageCleared)
      (else
        (Development|PrintString "웨이브 데이터를 불러올 수 없는 오류!" true true "(R=1.000000,G=0.000000,B=0.000000,A=1.000000)")))))

(event Custom|UnpauseWave
  (Development|PrintString "WaveManager - UnpauseWave()")
  (Utilities|Time|UnpauseTimerbyHandle (Variables|Default|GetWaveTimer)))

(event Custom|SetNextWaveInfo
  (Math|Integer|IncrementInt (Variables|Default|GetCurrentWaveIndex)
    (:%20%20
      (CallFunction|SetWaveInfo))))

(event Custom|PrintRemainingTime
  (bind _intermissiontimer (Variables|Default|GetIntermissionTimer))
  (bind _returnvalue (Utilities|Time|GetTimerRemainingTimebyHandle _intermissiontimer))
  (if (< _returnvalue 0.0)
    (Utilities|Time|ClearandInvalidateTimerbyHandle (stale Custom|StartIntermission _returnvalue_2))
    (elif (< _returnvalue 3.0)
      (Development|PrintString (Utilities|String|BuildString(Integer) "" "남은 쉬는 시간 : " (Math|Float|Round _returnvalue))))))

(event EventTick
  (params (DeltaSeconds :type Float%20%28single-precision%29))
  (if (>= (Variables|Default|GetCurrentWaveIndex) (- (Variables|Default|GetTotalWaveCount) 1))
    (bind _output_get (Variables|Default|SetElapsedTime (+ (Variables|Default|GetElapsedTime) DeltaSeconds)))
    (if (>= _output_get 1.0)
      (Variables|Default|SetElapsedTime 0.0)
      (bind _result (Math|Float|IncrementFloat (Variables|Default|GetLastWaveElapsedTime))
        (:%20%20
          (Default|CallOnLastWaveElapsedTimeUpdate _result)
          (if (> _result 6e+01)
            (Class|BPIStageGameMode|StageFailed(Message) (Game|GetGameMode))))))))

(event Input|KeyboardEvents|DebugKey2
  (params (Key :type Key%20Structure :default "None") (ActionValue :type Input%20Action%20Value%20Structure))
  (:Pressed
    (Development|PrintString "WaveManager - StopWave()")
    (Utilities|Time|ClearandInvalidateTimerbyHandle (Variables|Default|GetWaveTimer))))

(event Input|KeyboardEvents|DebugKey3
  (params (Key :type Key%20Structure :default "None") (ActionValue :type Input%20Action%20Value%20Structure))
  (:Pressed
    (Development|PrintString "WaveManager - PauseWave()")
    (Utilities|Time|PauseTimerbyHandle (Variables|Default|GetWaveTimer))))

(event Input|KeyboardEvents|DebugKey4
  (params (Key :type Key%20Structure :default "None") (ActionValue :type Input%20Action%20Value%20Structure))
  (:Pressed
    (Development|PrintString "WaveManager - UnpauseWave()")
    (Utilities|Time|UnpauseTimerbyHandle (Variables|Default|GetWaveTimer))))

(event Input|KeyboardEvents|DebugKey1
  (params (Key :type Key%20Structure :default "None") (ActionValue :type Input%20Action%20Value%20Structure))
  (:Pressed
    (Development|PrintString (Utilities|String|BuildString(Integer) "" "Wave " (+ (Variables|Default|GetCurrentWaveIndex) 1) " 시작"))
    (CallFunction|SpawnMonster)
    (bind _returnvalue (Utilities|Time|SetTimerbyEvent (EventDispatchers|CreateEvent :!event Custom|SpawnMonster) (Variables|Default|GetCurrentWaveInterval) true))
    (Variables|Default|SetWaveTimer _returnvalue)))

(fn ConstructionScript)

(fn CheckStageCleared
  (if (and (Variables|Default|GetbWaveFinished) (<= (Variables|Default|GetMonsterCount) 0))
    (Class|BPIStageGameMode|StageCleared(Message) (Game|GetGameMode))))

(fn CheckStageFailed
  (if (> (Variables|Default|GetMonsterCount) (Variables|Default|GetMonsterCountLimit))
    (Class|BPIStageGameMode|StageFailed(Message) (Game|GetGameMode))))

(fn GetWavePhase
  (return (/ (Variables|Default|GetCurrentWaveIndex) 4)))