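; Component on the shop manager that auto-merges three matching towers into one tower of the next level.
; Each added tower triggers a scan of owned towers for the same name and level.
; On a match, data table rows keyed by name and level give the next tier, the matches are removed, and the factory spawns the upgrade on a free bench.
; The upgrade is re-added through AddTower, so merges can chain.
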(event `AddTower`
  (params (InTower :type "Actor Object Reference"))
  (`KismetArrayLibrary.Array_Add` (`self.Towers`) InTower)
  (bind _outtowername (message `/Game/Blueprints/Interface/BPI_Tower.GetTowerName` InTower))
  (set `self.CurrentTowerName` _outtowername)
  (bind _outtowerlevel (message `/Game/Blueprints/Interface/BPI_Tower.GetTowerLevel` InTower))
  (set `self.CurrentTowerLevel` _outtowerlevel)
  (`self.CheckLevelUp`))

(event `CheckLevelUp`
  (`KismetArrayLibrary.Array_Clear` (`self.CurrentMergedTowers`))
  (for _array_element (`self.Towers`)
    (bind _outtowername (message `/Game/Blueprints/Interface/BPI_Tower.GetTowerName` _array_element))
    (if (`KismetTextLibrary.EqualEqual_TextText` _outtowername (`self.CurrentTowerName`))
      (bind _outtowerlevel (message `/Game/Blueprints/Interface/BPI_Tower.GetTowerLevel` _array_element))
      (if (== _outtowerlevel (`self.CurrentTowerLevel`))
        (`KismetArrayLibrary.Array_Add` (`self.CurrentMergedTowers`) _array_element))))
  (if (>= (`KismetArrayLibrary.Array_Length` (`self.CurrentMergedTowers`)) 3)
    (`self.MergeTowers` (`KismetStringLibrary.Conv_StringToName` (`KismetStringLibrary.Concat_StrStr` (`KismetTextLibrary.Conv_TextToString` (`self.CurrentTowerName`)) "_" (`KismetStringLibrary.Conv_IntToString` (`self.CurrentTowerLevel`)))))))

(event `MergeTowers`
  (params (InTowerName :type Name))
  (bind _asbp_shop_manager (cast `/Game/Blueprints/Game/BP_ShopManager` (`self.GetOwner`)))
  (bind _returnvalue (`|GetDataTableRow` (`/Game/Blueprints/Game/BP_ShopManager.TowerDataTable` _asbp_shop_manager) InTowerName)
    (:`then`
      (bind _returnvalue_2 (`|GetDataTableRow` (`/Game/Blueprints/Game/BP_ShopManager.TowerDataTable` _asbp_shop_manager) (`.NextLevelTowerDataRowName_29_927D2E03438FCE8CC850A3A6FCDCDAE8` (break `/Game/Blueprints/Data/Tower/ST_TowerCommonData` (`.CommonData_10_6D5FFF6E49DF166C6B4E1F8BFED53BED` (break `/Game/Blueprints/Data/Tower/ST_TowerData` _returnvalue)))))
        (:`then`
          (for _array_element (`self.CurrentMergedTowers`)
            (`KismetArrayLibrary.Array_RemoveItem` (`self.Towers`) _array_element)
            (message `/Game/Blueprints/Interface/BPI_Tower.RemoveFromGame` _array_element))
          (bind _outgridmanager (`/Game/Blueprints/Frameworks/BFL_StageFunctionLibrary.GetGridManager`))
          (bind _outbench (`/Game/Blueprints/Game/BP_GridManager.GetNextAvailableBench` _outgridmanager))
          (bind _outspawnedtower (`/Game/Blueprints/Game/BPC_TowerFactory.SpawnTower` (`/Game/Blueprints/Game/BP_ShopManager.BPC_TowerFactory` _asbp_shop_manager) _returnvalue_2 (`Actor.K2_GetActorLocation` _outbench)))
          (message `/Game/Blueprints/Interface/BPI_Grid.PlaceTower` _outbench _outspawnedtower)
          (`self.AddTower` _outspawnedtower))))))