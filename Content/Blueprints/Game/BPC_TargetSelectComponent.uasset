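; BPC_TargetSelectComponent picks up to a requested number of targets from a set of overlapping actors by priority type.
; SelectTargets keeps living BPI_Monster actors, plus any actor without that interface, as candidates.
; First and Last Overlapped index the set from either end.
; Highest and Lowest Hp repeatedly scan HP via interface messages and remove each pick, without resetting the best HP between passes.
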(fn `SelectTargets`
  (params (InOverlappingActors :type "Set of Actor Object Reference") (InTargetPriorityType :type "/Game/Blueprints/Data/E_TargetPriorityType Enum" :default "NewEnumerator0") (InTargetCount :type Integer))
  (returns (OutTargets :type "Array of Actor Object Reference"))
  (locals (OverlappingActors :type "Set of Actor Object Reference") (TargetableActors :type "Set of Actor Object Reference") (TargetPriorityType :type "/Game/Blueprints/Data/E_TargetPriorityType Enum") (TargetCount :type Integer) (TargetsLastIndex :type Integer) (CurrentTarget :type "Actor Object Reference") (Targets :type "Array of Actor Object Reference") (HighestHp :type "Float (double-precision)") (LowestHp :type "Float (double-precision)" :default 99999.0))
  (bind _currenttarget (`local.CurrentTarget`))
  (bind _targetableactors (`local.TargetableActors`))
  (bind _currenttarget_2 (`local.CurrentTarget`))
  (bind _targetableactors_2 (`local.TargetableActors`))
  (bind _targetableactors_3 (`local.TargetableActors`))
  (bind _targetableactors_4 (`local.TargetableActors`))
  (`|ExecutionSequence`
    (:`then_0`
      (set `local.OverlappingActors` InOverlappingActors))
    (:`then_1`
      (set `local.TargetPriorityType` InTargetPriorityType))
    (:`then_2`
      (bind _output_get (set `local.TargetCount` InTargetCount))
      (set `local.TargetsLastIndex` (- _output_get 1))
      (bind _valuepin (`|SetForEach` (`local.OverlappingActors`))
        (:`then`
          (if (`KismetSystemLibrary.DoesImplementInterface` _valuepin "/Game/Blueprints/Interface/BPI_Monster.BPI_Monster_C")
            (bind _outisalive (message `/Game/Blueprints/Interface/BPI_Monster.IsAlive` _valuepin))
            (if _outisalive
              (`BlueprintSetLibrary.Set_Add` (`local.TargetableActors`) _valuepin :!label _label))
            (else
              (goto _label))))
        (:`CompletedPin`
          (switch `/Game/Blueprints/Data/E_TargetPriorityType` (`local.TargetPriorityType`)
            (:`NewEnumerator0`
              (for _index (range (+ (`local.TargetsLastIndex`) 1))
                (`KismetArrayLibrary.Array_Add` (`local.Targets`) (`BlueprintSetLibrary.Set_GetItemByIndex` _targetableactors_3 _index))
                (if (== (`BlueprintSetLibrary.Set_GetLastIndex` _targetableactors_3) _index)
                  (break)))
              (return (`local.Targets`)))
            (:`NewEnumerator1`
              (for _index_2 (range (+ (`local.TargetsLastIndex`) 1))
                (`KismetArrayLibrary.Array_Add` (`local.Targets`) (`BlueprintSetLibrary.Set_GetItemByIndex` _targetableactors_4 (- (`BlueprintSetLibrary.Set_GetLastIndex` _targetableactors_4) _index_2)))
                (if (== (`BlueprintSetLibrary.Set_GetLastIndex` (`local.TargetableActors`)) _index_2)
                  (break)))
              (return (`local.Targets`)))
            (:`NewEnumerator2`
              (for _ (range (+ (`local.TargetsLastIndex`) 1))
                (bind _valuepin_2 (`|SetForEach` (`local.TargetableActors`))
                  (:`then`
                    (bind _outhp (message `/Game/Blueprints/Interface/BPI_Monster.GetHp` _valuepin_2))
                    (if (> _outhp (`local.HighestHp`))
                      (set `local.CurrentTarget` _valuepin_2)
                      (set `local.HighestHp` _outhp)))
                  (:`CompletedPin`
                    (`KismetArrayLibrary.Array_Add` (`local.Targets`) _currenttarget_2)
                    (`BlueprintSetLibrary.Set_Remove` _targetableactors_2 _currenttarget_2)
                    (if (`BlueprintSetLibrary.Set_IsEmpty` _targetableactors_2)
                      (break)))))
              (return (`local.Targets`)))
            (:`NewEnumerator3`
              (for _ (range (+ (`local.TargetsLastIndex`) 1))
                (bind _valuepin_3 (`|SetForEach` (`local.TargetableActors`))
                  (:`then`
                    (bind _outhp_2 (message `/Game/Blueprints/Interface/BPI_Monster.GetHp` _valuepin_3))
                    (if (< _outhp_2 (`local.LowestHp`))
                      (set `local.CurrentTarget` _valuepin_3)
                      (set `local.LowestHp` _outhp_2)))
                  (:`CompletedPin`
                    (`KismetArrayLibrary.Array_Add` (`local.Targets`) _currenttarget)
                    (`BlueprintSetLibrary.Set_Remove` _targetableactors _currenttarget)
                    (if (`BlueprintSetLibrary.Set_IsEmpty` _targetableactors)
                      (break)))))
              (return (`local.Targets`)))))))))