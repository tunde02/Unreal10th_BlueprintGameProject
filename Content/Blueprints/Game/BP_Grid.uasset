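; BP_Grid is a single grid cell that holds a placed tower, identified by its row and column.
; Placing a tower stores it, sends it a place message with the cell and its bench flag, and turns the cube red.
; Removing the tower clears the reference and turns the cube green.
; Getters expose the coordinates, occupancy and world location of a snap point.
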(event `/Game/Blueprints/Interface/BPI_Grid.SetGridRowColumn`
  (params (InRow :type Integer) (InColumn :type Integer))
  (set `self.Row` InRow)
  (set `self.Column` InColumn))

(event `/Game/Blueprints/Interface/BPI_Grid.PlaceTower`
  (params (InTower :type "Actor Object Reference"))
  (bind _output_get (set `self.Tower` InTower))
  (message `/Game/Blueprints/Interface/BPI_Tower.Place` _output_get (`self.bIsBench`) self)
  (set `self.bHasTower` true)
  (`PrimitiveComponent.SetMaterial` (`self.Cube`) 0 "/Game/Materials/M_Red.M_Red"))

(event `/Game/Blueprints/Interface/BPI_Grid.RemoveTower`
  (`|ExecutionSequence`
    (:`then_0`
      (set `self.Tower` null))
    (:`then_1`
      (set `self.bHasTower` false))
    (:`then_2`
      (`PrimitiveComponent.SetMaterial` (`self.Cube`) 0 "/Game/Materials/M_Green.M_Green"))))

(fn `GetGridRowColumn`
  (returns (OutRow :type Integer) (OutColumn :type Integer))
  (return (`self.Row`) (`self.Column`)))

(fn `GetSnapLocation`
  (returns (OutLocation :type "Vector Structure"))
  (return (`SceneComponent.K2_GetComponentLocation` (`self.SnapLocation`))))

(fn `HasTower`
  (returns (OutHasTower :type Boolean))
  (return (`self.bHasTower`)))

(fn `UserConstructionScript`)