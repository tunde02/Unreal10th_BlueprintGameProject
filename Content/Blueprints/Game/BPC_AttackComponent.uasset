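; Actor component that carries out an attack from supplied attack data, targets, damage, pierce count and spawn point.
; Attack caches its inputs, then switches on attack type, with only the Projectile case implemented.
; That case spawns one projectile per valid target and initializes it through a message with the target's current location and attack stats.
; Radial damage calls and an older setter-based projectile setup remain unconnected.
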(fn `Attack`
  (params (InAttackData :type "/Game/Blueprints/Data/Tower/ST_AttackData Structure") (InTargets :type "Array of Actor Object Reference") (InDamage :type "Float (double-precision)") (InPierceCount :type Integer) (InProjectileSpawnPoint :type "Vector Structure"))
  (locals (Targets :type "Array of Actor Object Reference") (AttackType :type "/Game/Blueprints/Data/E_AttackType Enum") (ProjectileClass :type "/Game/Blueprints/Game/BP_Projectile Class Reference") (ProjectileSpeed :type "Float (double-precision)") (DamageRadius :type "Float (double-precision)") (AttackEffects :type "Array of /Game/Blueprints/Data/Effect/ST_EffectData Structure") (Damage :type "Float (double-precision)") (PierceCount :type Integer) (ProjectileSpawnPoint :type "Vector Structure") (SpawnedProjectile :type "/Game/Blueprints/Game/BP_Projectile Object Reference"))
  (bind (_attacktype _projectile _projectilespeed _damageradius _attackeffects) (break `/Game/Blueprints/Data/Tower/ST_AttackData` InAttackData))
  (`|ExecutionSequence`
    (:`then_0`
      (set `local.AttackType` _attacktype))
    (:`then_1`
      (set `local.ProjectileClass` _projectile))
    (:`then_2`
      (set `local.ProjectileSpeed` _projectilespeed))
    (:`then_3`
      (set `local.DamageRadius` _damageradius))
    (:`then_4`
      (set `local.AttackEffects` _attackeffects))
    (:`then_5`
      (set `local.Targets` InTargets))
    (:`then_6`
      (set `local.Damage` InDamage))
    (:`then_7`
      (set `local.PierceCount` InPierceCount))
    (:`then_8`
      (set `local.ProjectileSpawnPoint` InProjectileSpawnPoint)
      (switch `/Game/Blueprints/Data/E_AttackType` (`local.AttackType`)
        (:`NewEnumerator0`
          (for _array_element (`local.Targets`)
            (`/Engine/EditorBlueprintResources/StandardMacros.IsValid` _array_element
              (:`Is Valid`
                (bind _returnvalue (`|SpawnActorFromClass` (`local.ProjectileClass`) (`KismetMathLibrary.Conv_VectorToTransform` (`local.ProjectileSpawnPoint`)) "Undefined" "MultiplyWithRoot" null null))
                (message `/Game/Blueprints/Interface/BPI_Projectile.Initialize` _returnvalue (`Actor.K2_GetActorLocation` _array_element) (`local.Damage`) (`local.ProjectileSpeed`) (`local.PierceCount`) (`local.AttackEffects`))))))))))