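; Grid manager that holds the grid cells and bench slots used for tower placement.
; On BeginPlay it registers itself through SetGridManager.
; Lookup functions map a row and column to an entry in the flat Grids or Benches array, using ColumnSize as the stride for both.
; GetNextAvailableBench scans the benches in order and returns the first one whose HasTower message reports no tower.
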(event `self.ReceiveBeginPlay`
  (`/Game/Blueprints/Frameworks/BFL_GridFunctionLibrary.SetGridManager` self))

(fn `GetBenchByRowColumn`
  (params (InRow :type Integer) (InColumn :type Integer))
  (returns (OutBench :type "Actor Object Reference"))
  (locals (ColumnSize :type Integer :default 2))
  (return (`|GetArrayItem` (`self.Benches`) (+ (* InRow (`local.ColumnSize`)) InColumn))))

(fn `GetGridByRowColumn`
  (params (InRow :type Integer) (InColumn :type Integer))
  (returns (OutGrid :type "Actor Object Reference"))
  (locals (ColumnSize :type Integer))
  (return (`|GetArrayItem` (`self.Grids`) (+ (* InRow (`local.ColumnSize`)) InColumn))))

(fn `GetNextAvailableBench`
  (returns (OutBench :type "Actor Object Reference"))
  (for _array_element (`self.Benches`)
    (bind _outhastower (message `/Game/Blueprints/Interface/BPI_Grid.HasTower` _array_element))
    (if (not _outhastower)
      (return _array_element))))

(fn `UserConstructionScript`)