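; Support tower for a tower-defense game that buffs other placed towers within range instead of attacking.
; SetTowerData builds runtime stats, range sphere and effect map from tower data; Place snaps it to a grid, enabling the collider off the bench.
; Overlaps switch Tick on and off, and Tick sends the effects to placed towers every attack interval, with debug-drawn range and links.
; Selling refunds coins and removes it through the tower manager.
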(event `self.SetTowerData`
  (params (InTowerData :type "/Game/Blueprints/Data/Tower/ST_TowerData Structure"))
  (bind _output_get (set `self.TowerData` InTowerData))
  (`self.InternalSetTowerData` _output_get)
  (`self.SetActorTickEnabled` false)
  (`PrimitiveComponent.SetCollisionEnabled` (`self.RangeCollider`) "NoCollision"))

(event `self.Place`
  (params (InIsBench :type Boolean) (InGrid :type "Actor Object Reference"))
  (`|ExecutionSequence`
    (:`then_0`
      (bind _output_get (set `self.bIsPlaced` (not InIsBench)))
      (if _output_get
        (`PrimitiveComponent.SetCollisionEnabled` (`self.RangeCollider`) "QueryOnly")))
    (:`then_1`
      (set `self.Grid` InGrid))
    (:`then_2`
      (bind _outlocation (message `/Game/Blueprints/Interface/BPI_Grid.GetSnapLocation` (`self.Grid`)))
      (`self.K2_SetActorLocation` _outlocation))))

(event `self.Sell`
  (`/Game/Blueprints/Frameworks/BFL_StageFunctionLibrary.AddCoin` (`.Price_13_700F79AE49EBE6A72A9F8CA02F362021` (break `/Game/Blueprints/Data/Tower/ST_TowerCommonData` (`.CommonData_10_6D5FFF6E49DF166C6B4E1F8BFED53BED` (break `/Game/Blueprints/Data/Tower/ST_TowerData` (`self.TowerData`))))))
  (`self.RemoveFromGame`))

(event `self.RemoveFromGame`
  (message `/Game/Blueprints/Interface/BPI_Grid.RemoveTower` (`self.Grid`))
  (bind _outtowermanager (`/Game/Blueprints/Frameworks/BFL_StageFunctionLibrary.GetTowerManager`))
  (`/Game/Blueprints/Game/BP_TowerManager.DestroyTower` _outtowermanager self))

(event `SelectTarget`
  (set `self.CurrentTarget` (`BlueprintSetLibrary.Set_GetItemByIndex` (`self.OverlappingTowers`))))

(event `self.RangeCollider.OnComponentBeginOverlap`
  (params (OverlappedComponent :type "PrimitiveComponent Object Reference") (OtherActor :type "Actor Object Reference") (OtherComp :type "PrimitiveComponent Object Reference") (OtherBodyIndex :type Integer) (bFromSweep :type Boolean) (SweepResult :type "HitResult Structure (by ref)"))
  (`BlueprintSetLibrary.Set_Add` (`self.OverlappingTowers`) OtherActor)
  ; 주변의 적들이 하나 이상이고,
  ; 맵에 배치되었을 때만 틱 활성화
  (if (and (`self.bIsPlaced`) (>= (`BlueprintSetLibrary.Set_Length` (`self.OverlappingTowers`)) 1))
    (`self.SetActorTickEnabled` true)))

(event `self.RangeCollider.OnComponentEndOverlap`
  (params (OverlappedComponent :type "PrimitiveComponent Object Reference") (OtherActor :type "Actor Object Reference") (OtherComp :type "PrimitiveComponent Object Reference") (OtherBodyIndex :type Integer))
  (`BlueprintSetLibrary.Set_Remove` (`self.OverlappingTowers`) OtherActor)
  ; 주변에 적이 없으면 틱 비활성화
  (if (== 0 (`BlueprintSetLibrary.Set_Length` (`self.OverlappingTowers`)))
    (`self.SetActorTickEnabled` false)))

(event `self.ReceiveTick`
  (params (DeltaSeconds :type "Float (single-precision)"))
  (`self.DrawDebugRangeCircle`)
  (`self.TryEnchant`))

(event `TryEnchant`
  ; 현재 게임 시간이 인챈트 가능한 시간을 초과했을 경우에만 인챈트
  (if (> (`KismetSystemLibrary.GetGameTimeInSeconds`) (`self.NextEnchantableTime`))
    (`self.Enchant`)))

(event `Enchant`
  (bind _valuepin (`|SetForEach` (`self.OverlappingTowers`))
    (:`then`
      (`/Engine/EditorBlueprintResources/StandardMacros.IsValid` _valuepin
        (:`Is Valid`
          (bind _outisplaced (message `/Game/Blueprints/Interface/BPI_Tower.IsPlaced` _valuepin))
          (if _outisplaced
            ; 인챈트 이펙트 구현 부분
            (`self.DrawDebugLineToTarget` _valuepin)
            ; 타워가 가진 버프 효과들을 다른 타워들에게 추가
            (bind (_keypin _valuepin_2) (`|MapForEach` (`self.EnchantEffectMap`))
              (:`then`
                (message `/Game/Blueprints/Interface/BPI_EnchantEffectReceiver.AddEnchantEffect` _valuepin _keypin _valuepin_2))
              (:`CompletedPin`
                ; 다음 버프 가능한 시간 갱신
                (bind _outattackinterval (`self.GetAttackInterval`))
                (set `self.NextEnchantableTime` (+ _outattackinterval (`KismetSystemLibrary.GetGameTimeInSeconds`)))))))))))

(fn `DrawDebugLineToTarget`
  (params (InTargetTower :type "Actor Object Reference"))
  (bind _outattackinterval (`self.GetAttackInterval`))
  (`KismetSystemLibrary.DrawDebugLine` (`SceneComponent.K2_GetComponentLocation` (`self.Head`)) (`self.K2_GetActorLocation` InTargetTower) (struct :`R` 1.0 :`A` 1.0) _outattackinterval))

(fn `DrawDebugRangeCircle`
  (bind _outrange (`self.GetRange`))
  (`KismetSystemLibrary.DrawDebugCircle` (`self.K2_GetActorLocation`) _outrange 24 (struct :`R` 1.0 :`G` 1.0 :`B` 1.0 :`A` 1.0) 0.0 0.0 (1.0 0.0 0.0) (0.0 1.0 0.0)))

(fn `GetAttackInterval`
  (returns (OutAttackInterval :type "Float (double-precision)"))
  (return (/ 1.0 (`.Current_10_8823095F44368B8BD7DA00B9AF4F8038` (break `/Game/Blueprints/Data/Effect/ST_FloatStat` (`.AttackRate_29_2759D1F74AF0AA7105D4A6875A6697DD` (break `/Game/Blueprints/Data/Tower/ST_RuntimeTowerStatData` (`self.RuntimeStats`))))))))

(fn `GetAttackPower`
  (returns (OutAttackPower :type "Float (double-precision)"))
  (return (`.Current_10_8823095F44368B8BD7DA00B9AF4F8038` (break `/Game/Blueprints/Data/Effect/ST_FloatStat` (`.AttackPower_28_2FB15F5042532A850C5FCF81A6040443` (break `/Game/Blueprints/Data/Tower/ST_RuntimeTowerStatData` (`self.RuntimeStats`)))))))

(fn `GetNextLevelTowerDataRowName`
  (returns (OutNextLevelTowerDataRowName :type Name))
  (return (`.NextLevelTowerDataRowName_29_927D2E03438FCE8CC850A3A6FCDCDAE8` (break `/Game/Blueprints/Data/Tower/ST_TowerCommonData` (`.CommonData_10_6D5FFF6E49DF166C6B4E1F8BFED53BED` (break `/Game/Blueprints/Data/Tower/ST_TowerData` (`self.TowerData`)))))))

(fn `GetPlacedGrid`
  (returns (OutGrid :type "Actor Object Reference"))
  (return (`self.Grid`)))

(fn `GetRange`
  (returns (OutRange :type "Float (double-precision)"))
  (return (`.Current_10_8823095F44368B8BD7DA00B9AF4F8038` (break `/Game/Blueprints/Data/Effect/ST_FloatStat` (`.Range_30_9C4464FF40E92343355B06A8A01E3A59` (break `/Game/Blueprints/Data/Tower/ST_RuntimeTowerStatData` (`self.RuntimeStats`)))))))

(fn `GetTowerLevel`
  (returns (OutTowerLevel :type Integer))
  (return (`.Level_26_D8C49D9A459522A7AF834E834DE6B25C` (break `/Game/Blueprints/Data/Tower/ST_TowerCommonData` (`.CommonData_10_6D5FFF6E49DF166C6B4E1F8BFED53BED` (break `/Game/Blueprints/Data/Tower/ST_TowerData` (`self.TowerData`)))))))

(fn `GetTowerName`
  (returns (OutTowerName :type Text))
  (return (break `/Game/Blueprints/Data/Tower/ST_TowerCommonData` (`.CommonData_10_6D5FFF6E49DF166C6B4E1F8BFED53BED` (break `/Game/Blueprints/Data/Tower/ST_TowerData` (`self.TowerData`))))))

(fn `InternalSetTowerData`
  (params (InTowerData :type "/Game/Blueprints/Data/Tower/ST_TowerData Structure"))
  (locals (LocalAttackPower :type "Float (double-precision)") (LocalAttackRate :type "Float (double-precision)") (LocalRange :type "Float (double-precision)") (LocalTargetCount :type Integer) (LocalPierceCount :type Integer))
  (bind (_commondata _statdata _attackdata _auradata _enchantdata) (break `/Game/Blueprints/Data/Tower/ST_TowerData` InTowerData))
  (bind (_attackpower _attackrate _range _targetcount _piercecount) (break `/Game/Blueprints/Data/Tower/ST_TowerStatData` _statdata))
  (`|ExecutionSequence`
    (:`then_0`
      (set `local.LocalAttackPower` _attackpower))
    (:`then_1`
      (set `local.LocalAttackRate` _attackrate))
    (:`then_2`
      (set `local.LocalRange` _range))
    (:`then_3`
      (set `local.LocalTargetCount` _targetcount))
    (:`then_4`
      (set `local.LocalPierceCount` _piercecount))
    (:`then_5`
      (`SphereComponent.SetSphereRadius` (`self.RangeCollider`) (`local.LocalRange`) true)
      (set `self.RuntimeStats` (make `/Game/Blueprints/Data/Tower/ST_RuntimeTowerStatData` (make `/Game/Blueprints/Data/Effect/ST_FloatStat` (`local.LocalAttackPower`) (`local.LocalAttackPower`)) (make `/Game/Blueprints/Data/Effect/ST_FloatStat` (`local.LocalAttackRate`) (`local.LocalAttackRate`)) (make `/Game/Blueprints/Data/Effect/ST_FloatStat` (`local.LocalRange`) (`local.LocalRange`)) (make `/Game/Blueprints/Data/Effect/ST_IntStat` (`local.LocalTargetCount`) (`local.LocalTargetCount`)) (make `/Game/Blueprints/Data/Effect/ST_IntStat` (`local.LocalPierceCount`) (`local.LocalPierceCount`))))
      (`BlueprintMapLibrary.Map_Add` (`self.EnchantEffectMap`) (`.EffectType_29_192DAD4A459898673A1966BCF28039AD` (break `/Game/Blueprints/Data/Effect/ST_EffectData` (`.EnchantEffect_20_C1B0BAD0487CD8EA109814B0C806C8CC` (break `/Game/Blueprints/Data/Effect/ST_EnchantEffectData` _enchantdata)))) _enchantdata))))

(fn `IsPlaced`
  (returns (OutIsPlaced :type Boolean))
  (return (`self.bIsPlaced`)))

(fn `LookAtTarget`
  (params (DeltaTime :type "Float (single-precision)"))
  (`SceneComponent.K2_SetRelativeRotation` (`self.Head`) (`KismetMathLibrary.MakeRotator` 0.0 0.0 (.yaw (`KismetMathLibrary.RInterpTo` (`SceneComponent.K2_GetComponentRotation` (`self.Head`)) (`KismetMathLibrary.FindLookAtRotation` (`self.K2_GetActorLocation`) (`self.K2_GetActorLocation` (`self.CurrentTarget`))) DeltaTime 5.0))) false false)
  (return))

(fn `UserConstructionScript`)