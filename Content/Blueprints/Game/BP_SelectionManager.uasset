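; BP_SelectionManager tracks the currently selected tower or monster and broadcasts selection and data changes.
; Select sends select and deselect messages, moves stat-update bindings between actors, and treats reselecting the same actor as deselection.
; It also binds to the selected actor's destruction event.
; RefreshSelection rebroadcasts an actor's type and reference through OnSelectionDataUpdated.
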(fn `RefreshSelection`
  (params (InActor :type "Actor Object Reference"))
  (locals (CurrentSelectiedActor :type "Actor Object Reference"))
  (bind _outselectiontype (message `/Game/Blueprints/Interface/BPI_Selectable.GetSelectionType` InActor))
  (`self.OnSelectionDataUpdated` _outselectiontype InActor))

(fn `Select`
  (params (InActor :type "Actor Object Reference"))
  (locals (NewSelectedActor :type "Actor Object Reference"))
  (bind _currentselectedactor (`self.CurrentSelectedActor`))
  (set `local.NewSelectedActor` InActor)
  (`/Engine/EditorBlueprintResources/StandardMacros.IsValid` (`self.CurrentSelectedActor`)
    (:`Is Valid`
      (message `/Game/Blueprints/Interface/BPI_Selectable.OnDeselected` _currentselectedactor)
      (bind _outselectiontype (message `/Game/Blueprints/Interface/BPI_Selectable.GetSelectionType` _currentselectedactor))
      (switch `name` _outselectiontype
        (:`Tower`
          (bind _asbp_attack_tower (cast `/Game/Blueprints/Game/BP_AttackTower` (`self.CurrentSelectedActor`)))
          (remove `/Game/Blueprints/Game/BP_AttackTower.OnRuntimeStatUpdated` _asbp_attack_tower (`|CreateDelegate` :!event `RefreshSelection`)))
        (:`Monster`
          (bind _asbp_monster_base (cast `/Game/Blueprints/Game/BP_MonsterBase` (`self.CurrentSelectedActor`)))
          (remove `/Game/Blueprints/Game/BP_MonsterBase.OnRuntimeStatUpdated` _asbp_monster_base (`|CreateDelegate` :!event `RefreshSelection`))))
      (if (!= (`local.NewSelectedActor`) (`self.CurrentSelectedActor`))
        (bind _output_get (set `self.CurrentSelectedActor` (`local.NewSelectedActor`) :!label _label))
        (`/Engine/EditorBlueprintResources/StandardMacros.IsValid` _output_get
          (:`Is Valid`
            (message `/Game/Blueprints/Interface/BPI_Selectable.OnSelected` (`self.CurrentSelectedActor`))
            (bind _outselectiontype_2 (message `/Game/Blueprints/Interface/BPI_Selectable.GetSelectionType` (`self.CurrentSelectedActor`)))
            (switch `name` _outselectiontype_2
              (:`Tower`
                (bind _asbp_attack_tower_2 (cast `/Game/Blueprints/Game/BP_AttackTower` (`self.CurrentSelectedActor`)))
                (add `/Game/Blueprints/Game/BP_AttackTower.OnRuntimeStatUpdated` _asbp_attack_tower_2 (`|CreateDelegate` :!event `RefreshSelection`)))
              (:`Monster`
                (bind _asbp_monster_base_2 (cast `/Game/Blueprints/Game/BP_MonsterBase` (`self.CurrentSelectedActor`)))
                (add `/Game/Blueprints/Game/BP_MonsterBase.OnRuntimeStatUpdated` _asbp_monster_base_2 (`|CreateDelegate` :!event `RefreshSelection`))))
            (add `self.OnDestroyed` (`self.CurrentSelectedActor`) (`|CreateDelegate` :!event `Select`))
            (`self.OnSelectionChanged` _outselectiontype_2 (`self.CurrentSelectedActor`)))
          (:`Is Not Valid`
            (`self.OnSelectionChanged` "None" :!label _label_2)))
        (else
          (set `self.CurrentSelectedActor` null)
          (goto _label_2))))
    (:`Is Not Valid`
      (goto _label))))

(fn `UserConstructionScript`)