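; Tower manager that tracks placed towers and handles auto-battler style three-of-a-kind merging.
; New towers spawn through a tower factory on the next available bench from the grid manager, then register in the Towers list.
; Three matching name and level towers are replaced by their next-level data table row, spawned with sparks VFX.
; Merged spawns re-enter the same check, so upgrades chain recursively.
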(event `Initialize`
  (`KismetArrayLibrary.Array_Clear` (`self.Towers`)))

(event `RemoveTower`
  (params (InTower :type "Actor Object Reference"))
  (`KismetArrayLibrary.Array_RemoveItem` (`self.Towers`) InTower))

(event `DestroyTower`
  (params (InTower :type "Actor Object Reference"))
  (`KismetArrayLibrary.Array_RemoveItem` (`self.Towers`) InTower)
  (`self.K2_DestroyActor` InTower))

(fn `AddTower`
  (params (InTower :type "Actor Object Reference"))
  (returns (OutTower :type "Actor Object Reference"))
  (`KismetArrayLibrary.Array_Add` (`self.Towers`) InTower)
  (bind _outtowername (message `/Game/Blueprints/Interface/BPI_Tower.GetTowerName` InTower))
  (set `self.CurrentTowerName` _outtowername)
  (bind _outtowerlevel (message `/Game/Blueprints/Interface/BPI_Tower.GetTowerLevel` InTower))
  (set `self.CurrentTowerLevel` _outtowerlevel)
  (bind _outtower (`self.CheckLevelUp` InTower))
  (return _outtower))

(fn `CheckLevelUp`
  (params (InNewTower :type "Actor Object Reference"))
  (returns (OutTower :type "Actor Object Reference"))
  (`KismetArrayLibrary.Array_Clear` (`self.CurrentMergedTowers`))
  (for _array_element (`self.Towers`)
    (`/Engine/EditorBlueprintResources/StandardMacros.IsValid` _array_element
      (:`Is Valid`
        (bind _outtowername (message `/Game/Blueprints/Interface/BPI_Tower.GetTowerName` _array_element))
        (if (`KismetTextLibrary.EqualEqual_TextText` _outtowername (`self.CurrentTowerName`))
          (bind _outtowerlevel (message `/Game/Blueprints/Interface/BPI_Tower.GetTowerLevel` _array_element))
          (if (== _outtowerlevel (`self.CurrentTowerLevel`))
            (`KismetArrayLibrary.Array_Add` (`self.CurrentMergedTowers`) _array_element))))))
  (if (>= (`KismetArrayLibrary.Array_Length` (`self.CurrentMergedTowers`)) 3)
    (bind _outtower (`self.MergeTower` (`KismetStringLibrary.Conv_StringToName` (`KismetStringLibrary.Concat_StrStr` (`KismetTextLibrary.Conv_TextToString` (`self.CurrentTowerName`)) "_" (`KismetStringLibrary.Conv_IntToString` (`self.CurrentTowerLevel`))))))
    (return _outtower)
    (else
      (return InNewTower))))

(fn `MergeTower`
  (params (InTowerName :type Name))
  (returns (OutTower :type "Actor Object Reference"))
  (bind _returnvalue (`|GetDataTableRow` (`self.TowerDataTable`) InTowerName)
    (:`then`
      (bind _returnvalue_2 (`|GetDataTableRow` (`self.TowerDataTable`) (`.NextLevelTowerDataRowName_29_927D2E03438FCE8CC850A3A6FCDCDAE8` (break `/Game/Blueprints/Data/Tower/ST_TowerCommonData` (`.CommonData_10_6D5FFF6E49DF166C6B4E1F8BFED53BED` (break `/Game/Blueprints/Data/Tower/ST_TowerData` _returnvalue)))))
        (:`then`
          (for _array_element (`self.CurrentMergedTowers`)
            (`KismetArrayLibrary.Array_RemoveItem` (`self.Towers`) _array_element)
            (message `/Game/Blueprints/Interface/BPI_Tower.RemoveFromGame` _array_element))
          (bind _outtower (`self.SpawnTowerAtBenchByTowerData` _returnvalue_2 true))
          (return _outtower))))))

(fn `PlayMergeVFX`
  (params (InLocation :type "Vector Structure"))
  (`GameplayStatics.SpawnEmitterAtLocation` "/Game/ExternalAssets/Realistic_Starter_VFX_Pack_Vol2/Particles/Sparks/P_Sparks_G.P_Sparks_G" InLocation (struct) (0.7 0.7 0.7)))

(fn `SpawnTowerAtBenchByTowerData`
  (params (InTowerData :type "/Game/Blueprints/Data/Tower/ST_TowerData Structure") (bIsMerge :type Boolean))
  (returns (OutTower :type "Actor Object Reference"))
  (bind _outgridmanager (`/Game/Blueprints/Frameworks/BFL_StageFunctionLibrary.GetGridManager`))
  (bind _outbench (`/Game/Blueprints/Game/BP_GridManager.GetNextAvailableBench` _outgridmanager))
  (`/Engine/EditorBlueprintResources/StandardMacros.IsValid` _outbench
    (:`Is Valid`
      (bind _returnvalue (`self.K2_GetActorLocation` _outbench))
      (bind _outspawnedtower (`/Game/Blueprints/Game/BPC_TowerFactory.SpawnTower` (`self.BPC_TowerFactory`) InTowerData _returnvalue))
      (message `/Game/Blueprints/Interface/BPI_Grid.PlaceTower` _outbench _outspawnedtower)
      (bind _outtower (`self.AddTower` _outspawnedtower))
      (if bIsMerge
        (`self.PlayMergeVFX` _returnvalue))
      (return _outtower))
    (:`Is Not Valid`
      (`KismetSystemLibrary.PrintString` "대기석이 꽉 찼습니다!!" true true (struct :`R` 1.0 :`A` 1.0))
      (return null))))

(fn `UserConstructionScript`)