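; Base wave monster that follows waypoints, takes Defense-reduced damage, and notifies the wave manager on death.
; SetMonsterData sets HP, color and runtime stats; passing the last waypoint costs 1 HP and wraps the path.
; AddEffect stores timed effects by type for a looping timer that applies periodic poison and expires them.
; Stat modifiers rebuild MoveSpeed and Defense from base plus flat and percent bonuses; instant effects only print.
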(event `self.ReceiveBeginPlay`
  (bind _sphere (`self.Sphere`))
  (bind _returnvalue (`PrimitiveComponent.CreateDynamicMaterialInstance` _sphere 0 (`PrimitiveComponent.GetMaterial` _sphere 0) "None"))
  (set `self.BaseColorMID` _returnvalue)
  (bind _returnvalue_2 (`KismetSystemLibrary.K2_SetTimer` null "TickActiveEffectMap" (`self.EffectTick`) true))
  (bind _output_get (set `self.TickEffectMapTimer` _returnvalue_2)))

(event `/Game/Blueprints/Interface/BPI_WaypointMovable.StartMove`
  (set `self.bMoving` true))

(event `/Game/Blueprints/Interface/BPI_WaypointMovable.SetWaypoints`
  (params (InWaypoints :type "Array of Actor Object Reference (by ref)"))
  (set `self.Waypoints` InWaypoints))

(event `self.ReceiveTick`
  (params (DeltaSeconds :type "Float (single-precision)"))
  (if (`self.bMoving`)
    (`self.MoveToCurrentWaypoint` DeltaSeconds)))

(event `MoveToCurrentWaypoint`
  (params (InDeltaSeconds :type "Float (double-precision)"))
  (bind _outmovespeed (`self.GetMoveSpeed`))
  (`self.K2_SetActorLocation` (`KismetMathLibrary.VInterpTo_Constant` (`self.K2_GetActorLocation`) (`self.K2_GetActorLocation` (`|GetArrayItem` (`self.Waypoints`) (`self.CurrentWaypointIndex`))) InDeltaSeconds _outmovespeed))
  (`self.CheckWaypointIndex`))

(event `CheckWaypointIndex`
  (bind _returnvalue (`KismetArrayLibrary.Array_Length` (`self.Waypoints`)))
  (if (< (`KismetMathLibrary.Vector_Distance2DSquared` (`self.K2_GetActorLocation`) (`self.K2_GetActorLocation` (`|GetArrayItem` (`self.Waypoints`) (`self.CurrentWaypointIndex`)))) 5.0)
    (bind _result (`/Engine/EditorBlueprintResources/StandardMacros.IncrementInt` (`self.CurrentWaypointIndex`))
      (:`  `
        (if (>= _result _returnvalue)
          (bind _result_2 (`/Engine/EditorBlueprintResources/StandardMacros.DecrementFloat` (`self.Hp`))
            (:`  `
              (if (<= _result_2 0.0)
                (`self.CheckAlive`)
                (else
                  (set `self.CurrentWaypointIndex` (+ (mod (`self.CurrentWaypointIndex`) _returnvalue) 1)))))))))))

(event `/Game/Blueprints/Interface/BPI_Monster.SetMonsterData`
  (params (InMonsterData :type "/Game/Blueprints/Data/ST_MonsterData Structure"))
  ; TODO: Internal 방식으로 변경
  (bind _output_get (set `self.MonsterData` InMonsterData))
  (set `self.Name` (break `/Game/Blueprints/Data/ST_MonsterData` _output_get))
  (set `self.Hp` (`.Hp_10_C566F61A414DDE5E9470D9A9D8E61F9B` (break `/Game/Blueprints/Data/ST_MonsterData` _output_get)))
  (bind _output_get_2 (set `self.BaseColor` (`.BaseColor_20_4F7FC98141C8FA79543F8F9FE30A9415` (break `/Game/Blueprints/Data/ST_MonsterData` _output_get))))
  (`MaterialInstanceDynamic.SetVectorParameterValue` (`self.BaseColorMID`) "BaseColor" _output_get_2)
  (set `self.RuntimeStat` (make `/Game/Blueprints/Data/ST_RuntimeMonsterStatData` (make `/Game/Blueprints/Data/Effect/ST_FloatStat` (`.MoveSpeed_11_7DAEBC3B4477F772A0AB76BABDB14070` (break `/Game/Blueprints/Data/ST_MonsterData` _output_get)) (`.MoveSpeed_11_7DAEBC3B4477F772A0AB76BABDB14070` (break `/Game/Blueprints/Data/ST_MonsterData` _output_get))) (make `/Game/Blueprints/Data/Effect/ST_FloatStat` (`.Defense_12_64784C32434D24EE74739E8823FC1506` (break `/Game/Blueprints/Data/ST_MonsterData` _output_get)) (`.Defense_12_64784C32434D24EE74739E8823FC1506` (break `/Game/Blueprints/Data/ST_MonsterData` _output_get))))))

(event `self.ReceiveAnyDamage`
  (params (Damage :type "Float (single-precision)") (DamageType :type "DamageType Object Reference") (InstigatedBy :type "Controller Object Reference") (DamageCauser :type "Actor Object Reference"))
  (bind _outdamage (`self.CalculateDamage` Damage))
  (set `self.Hp` (- (`self.Hp`) _outdamage))
  (`self.CheckAlive`))

(event `/Game/Blueprints/Interface/BPI_Monster.AddEffect`
  (params (InEffectType :type "/Game/Blueprints/Data/Effect/E_EffectType Enum" :default "NewEnumerator0") (InEffectData :type "/Game/Blueprints/Data/Effect/ST_EffectData Structure"))
  (bind (_effecttype _effectcategory) (break `/Game/Blueprints/Data/Effect/ST_EffectData` InEffectData))
  (bind (_effecttype_2 _effectcategory_2 _effecttrigger _targetstat _modifiertype _value _duration _interval) (break `/Game/Blueprints/Data/Effect/ST_EffectData` InEffectData))
  (bind _tickeffectmaptimer (`self.TickEffectMapTimer`))
  (bind (_value_2 _returnvalue) (`BlueprintMapLibrary.Map_Find` (`self.ActiveEffectMap`) InEffectType))
  (if (`|EnumEquality` _effectcategory "NewEnumerator3")
    (`self.ApplyInstantEffect` InEffectData)
    (else
      (if _returnvalue
        (set `self.PrevElapsedTime` (`.ElapsedTime_41_585291424D65149AAE70D091B683176F` (break `/Game/Blueprints/Data/Effect/ST_EffectData` _value_2)))
        (else
          (set `self.PrevElapsedTime` 0.0)))
      (`BlueprintMapLibrary.Map_Add` (`self.ActiveEffectMap`) InEffectType (make `/Game/Blueprints/Data/Effect/ST_EffectData` _effecttype_2 _effectcategory_2 _effecttrigger _targetstat _modifiertype _value _duration _interval (`self.PrevElapsedTime`)))
      (switch `/Game/Blueprints/Data/Effect/E_EffectCategory` _effectcategory
        (:`NewEnumerator0`
          (`self.CalculateStats`))
        (:`NewEnumerator2`
          (if (`KismetSystemLibrary.K2_IsTimerPausedHandle` _tickeffectmaptimer)
            (`KismetSystemLibrary.K2_UnPauseTimerHandle` _tickeffectmaptimer)))))))

(fn `AddModifierToFloatStat`
  (params (InStat :type "/Game/Blueprints/Data/Effect/ST_FloatStat Structure") (InEffectData :type "/Game/Blueprints/Data/Effect/ST_EffectData Structure"))
  (returns (OutCalculatedStat :type "/Game/Blueprints/Data/Effect/ST_FloatStat Structure"))
  (bind (_effecttype _effectcategory _effecttrigger _targetstat _modifiertype _value) (break `/Game/Blueprints/Data/Effect/ST_EffectData` InEffectData))
  (bind (_base _current _flatmodifier _percentmodifier) (break `/Game/Blueprints/Data/Effect/ST_FloatStat` InStat))
  (bind (_base_2 _current_2 _flatmodifier_2) (break `/Game/Blueprints/Data/Effect/ST_FloatStat` InStat))
  (switch `/Game/Blueprints/Data/Effect/E_ModifierType` _modifiertype
    (:`NewEnumerator0`
      (return (make `/Game/Blueprints/Data/Effect/ST_FloatStat` _base_2 0.0 (+ _flatmodifier_2 _value))))
    (:`NewEnumerator1`
      (return (make `/Game/Blueprints/Data/Effect/ST_FloatStat` _base 0.0 0.0 (+ _percentmodifier _value))))))

(fn `ApplyInstantEffect`
  (params (InEffectData :type "/Game/Blueprints/Data/Effect/ST_EffectData Structure"))
  (`KismetSystemLibrary.PrintString` (`KismetStringLibrary.Concat_StrStr` "MonsterBase - ApplyInstantEffect() - " (`|GetEnumeratorNameAsString` (`.EffectType_29_192DAD4A459898673A1966BCF28039AD` (break `/Game/Blueprints/Data/Effect/ST_EffectData` InEffectData))))))

(fn `ApplyPeriodicEffect`
  (params (InEffectData :type "/Game/Blueprints/Data/Effect/ST_EffectData Structure"))
  (bind (_effecttype _effectcategory _effecttrigger _targetstat _modifiertype _value) (break `/Game/Blueprints/Data/Effect/ST_EffectData` InEffectData))
  (switch `/Game/Blueprints/Data/Effect/E_EffectType` _effecttype
    (:`NewEnumerator1`
      (set `self.Hp` (- (`self.Hp`) _value))
      (`self.CheckAlive`))))

(fn `CalculateAllStatCurrents`
  (bind (_movespeed _defense) (break `/Game/Blueprints/Data/ST_RuntimeMonsterStatData` (`self.RuntimeStat`)))
  (bind _outstatfloat (`self.CalculateStatFloatCurrent` _movespeed))
  (bind _outstatfloat_2 (`self.CalculateStatFloatCurrent` _defense))
  (bind _structout (setmembers `/Game/Blueprints/Data/ST_RuntimeMonsterStatData` :`StructRef` (`self.RuntimeStat`) :`MoveSpeed` _outstatfloat :`Defense` _outstatfloat_2))
  (set `self.RuntimeStat` _structout))

(fn `CalculateDamage`
  (params (InDamage :type "Float (double-precision)"))
  (returns (OutDamage :type "Float (double-precision)"))
  (bind _outdefense (`self.GetDefense`))
  (return (* InDamage (/ 100.0 (+ _outdefense 100.0)))))

(fn `CalculateStatFloatCurrent`
  (params (InStatFloat :type "/Game/Blueprints/Data/Effect/ST_FloatStat Structure"))
  (returns (OutStatFloat :type "/Game/Blueprints/Data/Effect/ST_FloatStat Structure"))
  (bind (_base _current _flatmodifier _percentmodifier) (break `/Game/Blueprints/Data/Effect/ST_FloatStat` InStatFloat))
  (return (make `/Game/Blueprints/Data/Effect/ST_FloatStat` _base (`KismetMathLibrary.FMax` (* (+ _base _flatmodifier) (+ _percentmodifier 1.0))))))

(fn `CalculateStats`
  (bind (_movespeed _defense) (break `/Game/Blueprints/Data/ST_RuntimeMonsterStatData` (`self.RuntimeStat`)))
  (bind (_movespeed_2 _defense_2) (break `/Game/Blueprints/Data/ST_RuntimeMonsterStatData` (`self.RuntimeStat`)))
  (set `self.RuntimeStat` (make `/Game/Blueprints/Data/ST_RuntimeMonsterStatData` (make `/Game/Blueprints/Data/Effect/ST_FloatStat` (break `/Game/Blueprints/Data/Effect/ST_FloatStat` _movespeed) (`.Current_10_8823095F44368B8BD7DA00B9AF4F8038` (break `/Game/Blueprints/Data/Effect/ST_FloatStat` _movespeed))) (make `/Game/Blueprints/Data/Effect/ST_FloatStat` (break `/Game/Blueprints/Data/Effect/ST_FloatStat` _defense) (`.Current_10_8823095F44368B8BD7DA00B9AF4F8038` (break `/Game/Blueprints/Data/Effect/ST_FloatStat` _defense)))))
  (bind (_keypin _valuepin) (`|MapForEach` (`self.ActiveEffectMap`))
    (:`then`
      (bind (_effecttype _effectcategory _effecttrigger _targetstat) (break `/Game/Blueprints/Data/Effect/ST_EffectData` _valuepin))
      (if (`|EnumEquality` _effectcategory "NewEnumerator0")
        (switch `/Game/Blueprints/Data/Effect/E_StatType` _targetstat
          (:`NewEnumerator5`
            (bind _outcalculatedstat (`self.AddModifierToFloatStat` _movespeed_2 _valuepin))
            (setmembers `/Game/Blueprints/Data/ST_RuntimeMonsterStatData` :`StructRef` (`self.RuntimeStat`) :`MoveSpeed` _outcalculatedstat :`Defense` (struct)))
          (:`NewEnumerator6`
            (bind _outcalculatedstat_2 (`self.AddModifierToFloatStat` _defense_2 _valuepin))
            (setmembers `/Game/Blueprints/Data/ST_RuntimeMonsterStatData` :`StructRef` (`self.RuntimeStat`) :`MoveSpeed` (struct) :`Defense` _outcalculatedstat_2)))))
    (:`CompletedPin`
      (`self.CalculateAllStatCurrents`))))

(fn `CheckAlive`
  (if (not (> (`self.Hp`) 0.0))
    (bind _outwavemanager (`/Game/Blueprints/Frameworks/BFL_StageFunctionLibrary.GetWaveManager`))
    (`/Game/Blueprints/Game/BP_WaveManager.OnMonsterDeath` _outwavemanager)
    (`self.K2_DestroyActor`)))

(fn `GetDefense`
  (returns (OutDefense :type "Float (double-precision)"))
  (return (`.Current_10_8823095F44368B8BD7DA00B9AF4F8038` (break `/Game/Blueprints/Data/Effect/ST_FloatStat` (`.Defense_9_B897704149F669C7A8FDD49A38D546D1` (break `/Game/Blueprints/Data/ST_RuntimeMonsterStatData` (`self.RuntimeStat`)))))))

(fn `GetMoveSpeed`
  (returns (OutMoveSpeed :type "Float (double-precision)"))
  (return (`.Current_10_8823095F44368B8BD7DA00B9AF4F8038` (break `/Game/Blueprints/Data/Effect/ST_FloatStat` (`.MoveSpeed_8_F8FE12E44868107843978FBFE3F77DCE` (break `/Game/Blueprints/Data/ST_RuntimeMonsterStatData` (`self.RuntimeStat`)))))))

(fn `TickActiveEffectMap`
  (locals (NewEffectData :type "/Game/Blueprints/Data/Effect/ST_EffectData Structure") (NewEffectType :type "/Game/Blueprints/Data/Effect/E_EffectType Enum") (NewEffectCategory :type "/Game/Blueprints/Data/Effect/E_EffectCategory Enum") (NewElapsedTime :type "Float (double-precision)") (NewTotalElapsedTime :type "Float (double-precision)") (CurrentDuration :type "Float (double-precision)") (CurrentInterval :type "Float (double-precision)") (bNeedRecalculate :type Boolean) (ExpiredEffectMap :type "Array of /Game/Blueprints/Data/Effect/E_EffectType Enum"))
  (bind (_keypin _valuepin) (`|MapForEach` (`self.ActiveEffectMap`))
    (:`then`
      (set `local.NewEffectType` _keypin)
      (bind _output_get (set `local.NewEffectData` _valuepin))
      (bind (_effecttype _effectcategory _effecttrigger _targetstat _modifiertype _value _duration _interval _elapsedtime _totalelapsedtime) (break `/Game/Blueprints/Data/Effect/ST_EffectData` _output_get))
      (set `local.NewEffectCategory` _effectcategory)
      (`|ExecutionSequence`
        (:`then_0`
          (set `local.CurrentDuration` _duration))
        (:`then_1`
          (set `local.CurrentInterval` _interval))
        (:`then_2`
          (if (`|EnumEquality` "NewEnumerator2" (`local.NewEffectCategory`))
            (set `local.NewElapsedTime` (+ _elapsedtime (`self.EffectTick`)))))
        (:`then_3`
          (set `local.NewTotalElapsedTime` (+ _totalelapsedtime (`self.EffectTick`)))
          (if (not (<= (`local.CurrentDuration`) (`local.NewTotalElapsedTime`)))
            (if (`|EnumEquality` "NewEnumerator2" (`local.NewEffectCategory`))
              (if (>= (`local.NewElapsedTime`) (`local.CurrentInterval`))
                ; 효과 발동 시간이 채워진 효과는 ApplyPeriodicEffect
                (bind _output_get_2 (set `local.NewElapsedTime` (- (`local.NewElapsedTime`) (`local.CurrentInterval`))))
                (bind _structout (setmembers `/Game/Blueprints/Data/Effect/ST_EffectData` :`StructRef` (`local.NewEffectData`) :`ElapsedTime` _output_get_2 :`TotalElapsedTime` (`local.NewTotalElapsedTime`)))
                (`BlueprintMapLibrary.Map_Add` (`self.ActiveEffectMap`) (`local.NewEffectType`) _structout)
                (`self.ApplyPeriodicEffect` _structout)
                (else
                  ; 아직 효과 발동 시간이 채워지지 않은 효과는 ElapsedTime만 갱신
                  (bind _structout_2 (setmembers `/Game/Blueprints/Data/Effect/ST_EffectData` :`StructRef` (`local.NewEffectData`) :`ElapsedTime` (`local.NewElapsedTime`) :`TotalElapsedTime` (`local.NewTotalElapsedTime`) :!label _label))
                  (`BlueprintMapLibrary.Map_Add` (`self.ActiveEffectMap`) (`local.NewEffectType`) _structout_2)))
              (else
                (goto _label)))
            (else
              ; 지속시간이 끝난 효과 저장
              (`KismetArrayLibrary.Array_Add` (`local.ExpiredEffectMap`) (`local.NewEffectType`)))))))
    (:`CompletedPin`
      ; 지속 시간이 끝난 효과들을 ActiveEffectMap에서 제거
      (for _array_element (`local.ExpiredEffectMap`)
        ;; 스탯 관련 효과는 지속시간이 끝나면 스탯을 다시 계산해야됨
        (if (`|EnumEquality` (`.EffectCategory_12_8B9226C74EA0972C36E0D19B1BE55C05` (break `/Game/Blueprints/Data/Effect/ST_EffectData` (`BlueprintMapLibrary.Map_Find` (`self.ActiveEffectMap`) _array_element))) "NewEnumerator0")
          (set `local.bNeedRecalculate` true))
        (`BlueprintMapLibrary.Map_Remove` (`self.ActiveEffectMap`) _array_element))
      (if (`local.bNeedRecalculate`)
        (`self.CalculateStats`)))))

(fn `UserConstructionScript`)