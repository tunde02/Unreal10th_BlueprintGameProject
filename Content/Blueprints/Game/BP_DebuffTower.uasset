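; BP_DebuffTower is a tower that applies debuff effects to monsters overlapping it.
; HandleSetTowerData extends the parent by storing the tower's AuraData in DebuffEffectMap, keyed by effect type.
; Action sends every mapped effect to each valid overlapping actor through AddEffectMessage, then updates the next available time.
; A debug line call marked as the effect visual is left disconnected.
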(fn `Action`
  (bind _valuepin (`|SetForEach` (`self.OverlappingActors`))
    (:`then`
      (`/Engine/EditorBlueprintResources/StandardMacros.IsValid` _valuepin
        (:`Is Valid`
          ; 타워가 가진 디버프 효과들을 몬스터에 추가
          (bind (_keypin _valuepin_2) (`|MapForEach` (`self.DebuffEffectMap`))
            (:`then`
              (message `/Game/Blueprints/Interface/BPI_Monster.AddEffect` _valuepin _keypin _valuepin_2))))))
    (:`CompletedPin`
      (`self.UpdateNextAvailableTime`))))

(fn `HandleSetTowerData`
  (params (InTowerData :type "/Game/Blueprints/Data/Tower/ST_TowerData Structure"))
  (bind (_commondata _statdata _attackdata _auradata) (break `/Game/Blueprints/Data/Tower/ST_TowerData` InTowerData))
  (`parent.HandleSetTowerData` InTowerData)
  (`BlueprintMapLibrary.Map_Add` (`self.DebuffEffectMap`) (`.EffectType_29_192DAD4A459898673A1966BCF28039AD` (break `/Game/Blueprints/Data/Effect/ST_EffectData` _auradata)) _auradata))

(fn `UserConstructionScript`
  (`parent.UserConstructionScript`))