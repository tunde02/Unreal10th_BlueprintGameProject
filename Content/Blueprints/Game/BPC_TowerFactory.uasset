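; Tower factory Blueprint that spawns tower actors at a given location and initializes them.
; SpawnTower takes the class from the passed tower info, then sends only the tower data to the new actor, as its tower-info message node is disconnected.
; SpawnTowerByName looks up a TowerDataTable row by name, spawns its TowerType and passes that row as tower info.
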(fn `SpawnTower`
  (params (InTowerInfo :type "/Game/Blueprints/Data/ST_TowerInfo Structure") (InLocation :type "Vector Structure") (InTowerData :type "/Game/Blueprints/Data/Tower/ST_TowerData Structure"))
  (returns (OutSpawnedTower :type "Actor Object Reference"))
  (bind _returnvalue (`|SpawnActorFromClass` (`.TowerType_18_AD44882C4F91A6C48C97BC91541001B8` (break `/Game/Blueprints/Data/ST_TowerInfo` InTowerInfo)) (`KismetMathLibrary.MakeTransform` InLocation) "Undefined" "MultiplyWithRoot" null null))
  (message `/Game/Blueprints/Interface/BPI_Tower.SetTowerData` _returnvalue InTowerData)
  (return _returnvalue))

(fn `SpawnTowerByName`
  (params (InName :type Name) (InLocation :type "Vector Structure"))
  (returns (OutSpawnedTower :type "Actor Object Reference"))
  (bind _returnvalue (`|GetDataTableRow` (`self.TowerDataTable`) InName)
    (:`then`
      (bind _returnvalue_2 (`|SpawnActorFromClass` (`.TowerType_18_AD44882C4F91A6C48C97BC91541001B8` (break `/Game/Blueprints/Data/ST_TowerInfo` _returnvalue)) (`KismetMathLibrary.MakeTransform` InLocation) "Undefined" "MultiplyWithRoot" null null))
      (message `/Game/Blueprints/Interface/BPI_Tower.SetTowerInfo` _returnvalue_2 _returnvalue)
      (return _returnvalue_2))
    (:`RowNotFound`
      (return null))))