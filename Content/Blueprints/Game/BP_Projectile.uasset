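; BP_Projectile is a projectile that damages monsters and applies attack effects to them, with support for piercing.
; It stays inert without collision until Initialize sets its damage, speed, pierce count and effects, launches it straight toward a target location and starts its lifespan.
; On overlap, BPI_Monster actors receive each effect, then damage, and use up one pierce.
; Any other overlap, or running out of pierces, destroys it.
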(event `self.ReceiveBeginPlay`
  (`PrimitiveComponent.SetCollisionEnabled` (`self.Sphere`) "NoCollision")
  (set `ProjectileMovementComponent.InitialSpeed` 0.0 (`self.ProjectileMovement`))
  (set `ProjectileMovementComponent.MaxSpeed` 0.0 (`self.ProjectileMovement`)))

(event `/Game/Blueprints/Interface/BPI_Projectile.Initialize`
  (params (InTargetLocation :type "Vector Structure") (InDamage :type "Float (double-precision)") (InProjectileSpeed :type "Float (double-precision)") (InPierceCount :type Integer) (InAttackEffects :type "Array of /Game/Blueprints/Data/Effect/ST_EffectData Structure (by ref)"))
  (`|ExecutionSequence`
    (:`then_0`
      (bind _output_get (set `self.TargetLocation` InTargetLocation)))
    (:`then_1`
      (set `self.Damage` InDamage))
    (:`then_2`
      (set `self.ProjectileSpeed` InProjectileSpeed))
    (:`then_3`
      (set `self.PierceCount` InPierceCount))
    (:`then_4`
      (set `self.AttackEffects` InAttackEffects)
      (set `ProjectileMovementComponent.InitialSpeed` (`self.ProjectileSpeed`) (`self.ProjectileMovement`))
      (set `ProjectileMovementComponent.MaxSpeed` (`self.ProjectileSpeed`) (`self.ProjectileMovement`))
      (set `MovementComponent.Velocity` (* (`KismetMathLibrary.Normal` (- _output_get (`self.K2_GetActorLocation`))) (`self.ProjectileSpeed`)) (`self.ProjectileMovement`))
      (`PrimitiveComponent.SetCollisionEnabled` (`self.Sphere`) "QueryOnly")
      (`self.SetLifeSpan` (`self.LifeSpan`)))))

(event `self.Sphere.OnComponentBeginOverlap`
  (params (OverlappedComponent :type "PrimitiveComponent Object Reference") (OtherActor :type "Actor Object Reference") (OtherComp :type "PrimitiveComponent Object Reference") (OtherBodyIndex :type Integer) (bFromSweep :type Boolean) (SweepResult :type "HitResult Structure (by ref)"))
  (bind _piercecount (`self.PierceCount`))
  (`/Engine/EditorBlueprintResources/StandardMacros.IsValid` OtherActor
    (:`Is Valid`
      (if (`KismetSystemLibrary.DoesImplementInterface` OtherActor "/Game/Blueprints/Interface/BPI_Monster.BPI_Monster_C")
        (for _array_element (`self.AttackEffects`)
          (message `/Game/Blueprints/Interface/BPI_Monster.AddEffect` OtherActor (`.EffectType_29_192DAD4A459898673A1966BCF28039AD` (break `/Game/Blueprints/Data/Effect/ST_EffectData` _array_element)) _array_element))
        (`GameplayStatics.ApplyDamage` OtherActor (`self.Damage`))
        (`/Engine/EditorBlueprintResources/StandardMacros.DecrementInt` _piercecount
          (:`  `
            (if (< _piercecount 0)
              (`self.K2_DestroyActor`))))
        (else
          (`self.K2_DestroyActor` :!label _label))))
    (:`Is Not Valid`
      (goto _label))))

(fn `UserConstructionScript`)