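; Shop manager that offers random towers in slots and handles coin-based purchases and rerolls.
; Refreshes roll each slot's grade from the current wave phase's probability row using cumulative thresholds, then pick a random tower of that grade at level 0 or below.
; Purchases spawn the tower on the bench through the tower manager, mark the slot sold and deduct coins.
; Refreshes and purchases broadcast slot updates; refreshes also clear locked and sold flags.
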(event `Initialize`
  (`KismetArrayLibrary.Array_Resize` (`self.ShopSlots`) (`self.SlotSize`))
  (`self.RefreshShopSlots`))

(event `RefreshShopSlots`
  (bind _shopslots (`self.ShopSlots`))
  (bind _outwavemanager (`/Game/Blueprints/Frameworks/BFL_StageFunctionLibrary.GetWaveManager`))
  (bind _outwavephase (`/Game/Blueprints/Game/BP_WaveManager.GetWavePhase` _outwavemanager))
  (for (_ _array_index) _shopslots
    (bind _outtowerdata (`self.GetRandomTowerData` (`KismetStringLibrary.Conv_StringToName` (`KismetStringLibrary.Concat_StrStr` "Phase" (`KismetStringLibrary.Conv_IntToString` _outwavephase)))))
    (`KismetArrayLibrary.Array_Set` _shopslots _array_index (make `/Game/Blueprints/Data/ST_ShopSlotInfo` _outtowerdata)))
  (`self.OnUpdateShopSlots` (`self.ShopSlots`)))

(event `Reroll`
  (bind _outcoin (`/Game/Blueprints/Frameworks/BFL_StageFunctionLibrary.GetCoin`))
  (bind _outcanbuy (`self.CanReroll` _outcoin (`self.RerollPrice`)))
  (if _outcanbuy
    (`self.RefreshShopSlots`)
    (`/Game/Blueprints/Frameworks/BFL_StageFunctionLibrary.SubtractCoin` (`self.RerollPrice`))
    (else
      (`KismetSystemLibrary.PrintString` "소지금이 부족해 리롤 불가능!!" true true (struct :`R` 1.0 :`A` 1.0)))))

(event `BuyTower`
  (params (InSlotIndex :type Integer))
  (bind _shopslots (`self.ShopSlots`))
  (bind _output (`|GetArrayItem` _shopslots InSlotIndex))
  ; 우선 타워를 구매할 수 있는지 검사
  (bind _outcoin (`/Game/Blueprints/Frameworks/BFL_StageFunctionLibrary.GetCoin`))
  (bind _outcanbuy (`self.CanBuyTower` _outcoin (`.Price_13_700F79AE49EBE6A72A9F8CA02F362021` (break `/Game/Blueprints/Data/Tower/ST_TowerCommonData` (`.CommonData_10_6D5FFF6E49DF166C6B4E1F8BFED53BED` (break `/Game/Blueprints/Data/Tower/ST_TowerData` (`.TowerData_12_EC9133A449A62FDF049D379F6A7A071C` (break `/Game/Blueprints/Data/ST_ShopSlotInfo` (`|GetArrayItem` (`self.ShopSlots`) InSlotIndex)))))))))
  (if _outcanbuy
    (bind _outtowermanager (`/Game/Blueprints/Frameworks/BFL_StageFunctionLibrary.GetTowerManager`))
    (bind _outtower (`/Game/Blueprints/Game/BP_TowerManager.SpawnTowerAtBenchByTowerData` _outtowermanager (`.TowerData_12_EC9133A449A62FDF049D379F6A7A071C` (break `/Game/Blueprints/Data/ST_ShopSlotInfo` (`|GetArrayItem` (`self.ShopSlots`) InSlotIndex)))))
    (`/Engine/EditorBlueprintResources/StandardMacros.IsValid` _outtower
      (:`Is Valid`
        ; 구매한 ShopSlot의
        ; bSold = true
        (setmembers `/Game/Blueprints/Data/ST_ShopSlotInfo` :`StructRef` _output :`bSold` true)
        (`self.OnUpdateShopSlots` _shopslots)
        (`/Game/Blueprints/Frameworks/BFL_StageFunctionLibrary.SubtractCoin` (`.Price_13_700F79AE49EBE6A72A9F8CA02F362021` (break `/Game/Blueprints/Data/Tower/ST_TowerCommonData` (`.CommonData_10_6D5FFF6E49DF166C6B4E1F8BFED53BED` (break `/Game/Blueprints/Data/Tower/ST_TowerData` (`.TowerData_12_EC9133A449A62FDF049D379F6A7A071C` (break `/Game/Blueprints/Data/ST_ShopSlotInfo` _output)))))))))
    (else
      (`KismetSystemLibrary.PrintString` "소지금이 부족합니다!!" true true (struct :`R` 1.0 :`A` 1.0)))))

(fn `CanBuyTower`
  (params (InCoin :type Integer) (InPrice :type Integer))
  (returns (OutCanBuy :type Boolean))
  (return (>= InCoin InPrice)))

(fn `CanReroll`
  (params (InCoin :type Integer) (InPrice :type Integer))
  (returns (OutCanBuy :type Boolean))
  (return (>= InCoin InPrice)))

(fn `GetRandomTowerData`
  (params (InPhase :type Name))
  (returns (OutTowerData :type "/Game/Blueprints/Data/Tower/ST_TowerData Structure"))
  (locals (TowersOfGradeLength :type Integer) (TowersOfGrade :type "Array of /Game/Blueprints/Data/Tower/ST_TowerData Structure") (CurrentGrade0Probability :type "Float (double-precision)") (CurrentGrade1Probability :type "Float (double-precision)") (CurrentGrade2Probability :type "Float (double-precision)") (CurrentGrade3Probability :type "Float (double-precision)") (CurrentProbability :type "Float (double-precision)") (CurrentThreshold :type "Float (double-precision)"))
  (bind _returnvalue (`|GetDataTableRow` (`self.ShopSlotProbabilityDataTable`) InPhase)
    (:`then`
      (`|ExecutionSequence`
        (:`then_0`
          (bind (_wavephase _grade0 _grade1 _grade2 _grade3) (break `/Game/Blueprints/Data/ST_ShopSlotProbability` _returnvalue))
          (set `local.CurrentGrade0Probability` _grade0))
        (:`then_1`
          (set `local.CurrentGrade1Probability` _grade1))
        (:`then_2`
          (set `local.CurrentGrade2Probability` _grade2))
        (:`then_3`
          (set `local.CurrentGrade3Probability` _grade3)
          (set `local.CurrentProbability` (`KismetMathLibrary.RandomFloat`))
          (set `local.CurrentThreshold` (`local.CurrentGrade0Probability`))
          (if (<= (`local.CurrentProbability`) (`local.CurrentThreshold`))
            (bind _outtowersofgrade (`self.GetTowersOfGrade` 0))
            (bind _output_get (set `local.TowersOfGrade` _outtowersofgrade))
            (set `local.TowersOfGradeLength` (`KismetMathLibrary.RandomIntegerInRange` 0 (- (`KismetArrayLibrary.Array_Length` _output_get) 1)))
            (return (`|GetArrayItem` (`local.TowersOfGrade`) (`local.TowersOfGradeLength`)))
            (else
              (set `local.CurrentThreshold` (+ (`local.CurrentGrade0Probability`) (`local.CurrentGrade1Probability`)))
              (if (<= (`local.CurrentProbability`) (`local.CurrentThreshold`))
                (bind _outtowersofgrade_2 (`self.GetTowersOfGrade` 1))
                (bind _output_get_2 (set `local.TowersOfGrade` _outtowersofgrade_2))
                (set `local.TowersOfGradeLength` (`KismetMathLibrary.RandomIntegerInRange` 0 (- (`KismetArrayLibrary.Array_Length` _output_get_2) 1)))
                (return (`|GetArrayItem` (`local.TowersOfGrade`) (`local.TowersOfGradeLength`)))
                (else
                  (set `local.CurrentThreshold` (+ (`local.CurrentGrade0Probability`) (`local.CurrentGrade1Probability`) (`local.CurrentGrade2Probability`)))
                  (if (<= (`local.CurrentProbability`) (`local.CurrentThreshold`))
                    (bind _outtowersofgrade_3 (`self.GetTowersOfGrade` 2))
                    (bind _output_get_3 (set `local.TowersOfGrade` _outtowersofgrade_3))
                    (set `local.TowersOfGradeLength` (`KismetMathLibrary.RandomIntegerInRange` 0 (- (`KismetArrayLibrary.Array_Length` _output_get_3) 1)))
                    (return (`|GetArrayItem` (`local.TowersOfGrade`) (`local.TowersOfGradeLength`)))
                    (else
                      (bind _outtowersofgrade_4 (`self.GetTowersOfGrade` 3))
                      (bind _output_get_4 (set `local.TowersOfGrade` _outtowersofgrade_4))
                      (set `local.TowersOfGradeLength` (`KismetMathLibrary.RandomIntegerInRange` 0 (- (`KismetArrayLibrary.Array_Length` _output_get_4) 1)))
                      (return (`|GetArrayItem` (`local.TowersOfGrade`) (`local.TowersOfGradeLength`))))))))))))))

(fn `GetTowersOfGrade`
  (params (InGrade :type Integer))
  (returns (OutTowersOfGrade :type "Array of /Game/Blueprints/Data/Tower/ST_TowerData Structure"))
  (locals (TowersOfGrade :type "Array of /Game/Blueprints/Data/Tower/ST_TowerData Structure"))
  (bind _outrownames (`DataTableFunctionLibrary.GetDataTableRowNames` (`self.TowerDataTable`)))
  (for _array_element _outrownames
    (bind _returnvalue (`|GetDataTableRow` (`self.TowerDataTable`) _array_element)
      (:`then`
        (bind (_name _grade _level) (break `/Game/Blueprints/Data/Tower/ST_TowerCommonData` (`.CommonData_10_6D5FFF6E49DF166C6B4E1F8BFED53BED` (break `/Game/Blueprints/Data/Tower/ST_TowerData` _returnvalue))))
        (if (and (== _grade InGrade) (<= _level 0))
          (`KismetArrayLibrary.Array_Add` (`local.TowersOfGrade`) _returnvalue)))))
  (return (`local.TowersOfGrade`)))

(fn `UserConstructionScript`)