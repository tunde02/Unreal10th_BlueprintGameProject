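; Blueprint function library giving global access to the stage's grid manager and its grid and bench queries.
; A setter and getter store and read the GridManager reference on the StageGameState.
; Lookups for a grid or bench by row and column, and for the next available bench, forward to that manager through message calls, apparently interface messages.
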(fn `GetBenchByRowColumn`
  (params (InRow :type Integer) (InColumn :type Integer))
  (returns (OutBench :type "Actor Object Reference"))
  (bind _gs_stagegamestate (`/Game/Blueprints/Frameworks/BFL_StageFunctionLibrary.StageGameState` null))
  (bind _outbench (message `/Game/Blueprints/Interface/BPI_GridManager.GetBenchByRowColumn` (`/Game/Blueprints/Frameworks/GS_StageGameState.GridManager` _gs_stagegamestate) InRow InColumn))
  (return _outbench))

(fn `GetGridByRowColumn`
  (params (InRow :type Integer) (InColumn :type Integer))
  (returns (OutGrid :type "Actor Object Reference"))
  (bind _gs_stagegamestate (`/Game/Blueprints/Frameworks/BFL_StageFunctionLibrary.StageGameState` null))
  (bind _outgrid (message `/Game/Blueprints/Interface/BPI_GridManager.GetGridByRowColumn` (`/Game/Blueprints/Frameworks/GS_StageGameState.GridManager` _gs_stagegamestate) InRow InColumn))
  (return _outgrid))

(fn `GetGridManager`
  (returns (OutGridManager :type "Actor Object Reference"))
  (bind _gs_stagegamestate (`/Game/Blueprints/Frameworks/BFL_StageFunctionLibrary.StageGameState` null))
  (return (`/Game/Blueprints/Frameworks/GS_StageGameState.GridManager` _gs_stagegamestate)))

(fn `GetNextAvailableBench`
  (returns (OutBench :type "Actor Object Reference"))
  (bind _gs_stagegamestate (`/Game/Blueprints/Frameworks/BFL_StageFunctionLibrary.StageGameState` null))
  (bind _outbench (message `/Game/Blueprints/Interface/BPI_GridManager.GetNextAvailableBench` (`/Game/Blueprints/Frameworks/GS_StageGameState.GridManager` _gs_stagegamestate)))
  (return _outbench))

(fn `SetGridManager`
  (params (InGridManager :type "Actor Object Reference"))
  (bind _gs_stagegamestate (`/Game/Blueprints/Frameworks/BFL_StageFunctionLibrary.StageGameState` null))
  (set `/Game/Blueprints/Frameworks/GS_StageGameState.GridManager` InGridManager _gs_stagegamestate))