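; Stage player controller that lets the player drag towers not yet marked as placed and drop them onto grid cells with the mouse.
; Left press picks the tower under the cursor via BPI_Tower, saving its location and grid.
; Tick moves it along a raised horizontal plane using cursor-ray intersection.
; Release traces past the tower, transferring it to an empty BPI_Grid cell or snapping it back.
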(event `self.ReceiveTick`
  (params (DeltaSeconds :type "Float (single-precision)"))
  (bind (_locationx _locationy) (`self.GetMousePosition`))
  (bind (_originaltowerlocation_x _originaltowerlocation_y _originaltowerlocation_z) (`KismetMathLibrary.BreakVector` (`self.OriginalTowerLocation`)))
  (bind (_worldlocation _worlddirection) (`self.DeprojectScreenPositionToWorld` _locationx _locationy))
  (if (`self.bDragging`)
    (`self.K2_SetActorLocation` (`self.SelectedTower`) (`.Intersection` (`KismetMathLibrary.LinePlaneIntersection_OriginNormal` _worldlocation (* _worlddirection (`self.TraceDistance`)) (`KismetMathLibrary.MakeVector` 0.0 0.0 (+ _originaltowerlocation_z (`self.DraggingHeight`))) (0.0 0.0 1.0))) false false)))

(event `Key|LeftMouseButton`
  (params (Key :type "Key Structure"))
  (bind (_hitresult _returnvalue) (`self.GetHitResultUnderCursorByChannel` "TraceTypeQuery1"))
  (bind (_locationx _locationy) (`self.GetMousePosition`))
  (bind (_worldlocation _worlddirection) (`self.DeprojectScreenPositionToWorld` _locationx _locationy))
  (bind (_bblockinghit _binitialoverlap _time _distance _location _impactpoint _normal _impactnormal _physmat _hitactor) (`GameplayStatics.BreakHitResult` _hitresult))
  (:`Pressed`
    (if _returnvalue
      (if (`KismetSystemLibrary.DoesImplementInterface` _hitactor "/Game/Blueprints/Interface/BPI_Tower.BPI_Tower_C")
        (bind _outisplaced (message `/Game/Blueprints/Interface/BPI_Tower.IsPlaced` _hitactor))
        (if (not _outisplaced)
          (`|ExecutionSequence`
            (:`then_0`
              (set `self.SelectedTower` _hitactor))
            (:`then_1`
              (set `self.OriginalTowerLocation` (`self.K2_GetActorLocation` _hitactor)))
            (:`then_2`
              (set `self.bDragging` true))
            (:`then_3`
              (bind _outgrid (message `/Game/Blueprints/Interface/BPI_Tower.GetPlacedGrid` _hitactor))
              (set `self.OriginalGrid` _outgrid)))))))
  (:`Released`
    (if (`self.bDragging`)
      (bind (_outhit _returnvalue_2) (`KismetSystemLibrary.LineTraceSingle` _worldlocation (* _worlddirection (`self.TraceDistance`)) "TraceTypeQuery1" false (`|MakeArray` (`self.SelectedTower`))))
      (if _returnvalue_2
        (bind (_bblockinghit_2 _binitialoverlap_2 _time_2 _distance_2 _location_2 _impactpoint_2 _normal_2 _impactnormal_2 _physmat_2 _hitactor_2) (`GameplayStatics.BreakHitResult` _outhit))
        (if (`KismetSystemLibrary.DoesImplementInterface` _hitactor_2 "/Game/Blueprints/Interface/BPI_Grid.BPI_Grid_C")
          (bind _outhastower (message `/Game/Blueprints/Interface/BPI_Grid.HasTower` _hitactor_2))
          (if (not _outhastower)
            (message `/Game/Blueprints/Interface/BPI_Grid.PlaceTower` _hitactor_2 (`self.SelectedTower`))
            (message `/Game/Blueprints/Interface/BPI_Grid.RemoveTower` (`self.OriginalGrid`))
            (else
              (`self.K2_SetActorLocation` (`self.SelectedTower`) (`self.OriginalTowerLocation`) false false :!label _label)))
          (else
            (goto _label)))
        (else
          (goto _label)))
      (`|ExecutionSequence`
        (:`then_0`
          (set `self.bDragging` false))
        (:`then_1`
          (set `self.SelectedTower` null))
        (:`then_2`
          (set `self.OriginalTowerLocation` (0.0 0.0 0.0)))
        (:`then_3`
          (set `self.OriginalGrid` null))))))

(fn `UserConstructionScript`)